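; Demo hovercraft pawn that passes player input to a HoverControllerBP component for movement, look, rotation, jumping and free-camera control.
; Tick spins four fan meshes at a frame-rate-independent rate and runs the controller's hover update for when the craft is not possessed.
; Number keys switch possession between this craft, Demo_Hovercraft1 and the surface-riding demo craft by possessing the first actor found of each class.
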(event EventTick
  (params (DeltaSeconds :type Float%20%28single-precision%29))
  ;[1 1 1] Tick Events
  (Utilities|FlowControl|Sequence
    (:then_0
      ;;[1 1 1] Spin Rotors
      (Transformation|AddLocalRotation (Variables|Default|GetHover_Fan4) (Math|Rotator|MakeRotator 0.0 0.0 (* (Utilities|Time|GetWorldDeltaSeconds) (Variables|Default|GetRotation%20Per%20Second) 3.6e+02)) false false))
    (:then_1
      ;;[1 1 1] Keep Actor Hovering While Not Possessed
      (Default|NotPossesedHoverTick (Variables|Default|GetHover_Controller_BP)))))

(event Input|AxisEvents|InputAxisRotateRight
  (params (AxisValue :type Float%20%28single-precision%29))
  ;[1 1 1] Movement Input Events
  (Default|RotateActorAxisInput (Variables|Default|GetHover_Controller_BP) AxisValue))

(event Input|AxisEvents|InputAxisLookUp
  (params (AxisValue :type Float%20%28single-precision%29))
  ;[1 1 1] Movement Input Events
  (Default|AddLookatDirection (Variables|Default|GetHover_Controller_BP) (stale Input|AxisEvents|InputAxisTurn AxisValue) AxisValue))

(event Input|AxisEvents|InputAxisTurn
  (params (AxisValue :type Float%20%28single-precision%29))
  ;[1 1 1] Movement Input Events
  (Default|AddLookatDirection (Variables|Default|GetHover_Controller_BP) AxisValue (stale Input|AxisEvents|InputAxisLookUp AxisValue)))

(event Input|AxisEvents|InputAxisMoveForward
  (params (AxisValue :type Float%20%28single-precision%29))
  ;[1 1 1] Movement Input Events
  (Default|AddForwardMovement (Variables|Default|GetHover_Controller_BP) AxisValue))

(event Input|AxisEvents|InputAxisMoveRight
  (params (AxisValue :type Float%20%28single-precision%29))
  ;[1 1 1] Movement Input Events
  (Default|AddSidewaysMovement (Variables|Default|GetHover_Controller_BP) AxisValue))

(event Input|KeyboardEvents|2
  (params (Key :type Key%20Structure :default "None"))
  ;[1 1 1] Change Current Actor
  (:Pressed
    (bind _outactors (Actor|GetAllActorsOfClass "Demo_Hovercraft2_BP_C"))
    (Pawn|Possess (Game|GetPlayerController 0) (Utilities|Array|Get(acopy) _outactors))))

(event Input|KeyboardEvents|SpaceBar
  (params (Key :type Key%20Structure :default "None"))
  ;[1 1 1] Make Actor Jump
  (:Pressed
    (Default|Jump (Variables|Default|GetHover_Controller_BP) 1.5e+03 false 0.0)))

(event Input|KeyboardEvents|1
  (params (Key :type Key%20Structure :default "None"))
  ;[1 1 1] Change Current Actor
  (:Pressed
    (bind _outactors (Actor|GetAllActorsOfClass "/Game/Hover_Controller/Blueprints/Demo_Hovercraft1_BP.Demo_Hovercraft1_BP_C"))
    (Pawn|Possess (Game|GetPlayerController 0) (Utilities|Array|Get(acopy) _outactors))))

(event Input|KeyboardEvents|3
  (params (Key :type Key%20Structure :default "None"))
  ;[1 1 1] Change Current Actor
  (:Pressed
    (bind _outactors (Actor|GetAllActorsOfClass "/Game/Hover_Controller/Blueprints/Demo_Hovercraft_Surface_Riding_BP.Demo_Hovercraft_Surface_Riding_BP_C"))
    (Pawn|Possess (Game|GetPlayerController 0) (Utilities|Array|Get(acopy) _outactors))))

(event Input|MouseEvents|RightMouseButton
  (params (Key :type Key%20Structure :default "None"))
  (bind _hover_controller_bp (Variables|Default|GetHover_Controller_BP))
  ;[1 1 1] Control Free Camera Rotaiton
  (:Pressed
    (Default|FreeCameraRotation _hover_controller_bp false))
  (:Released
    (Default|FreeCameraRotation _hover_controller_bp true)))

(fn ConstructionScript)