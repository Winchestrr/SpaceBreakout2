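; Player ship pawn that auto-moves forward, steers sideways and hovers over the surface beneath it, firing one bullet per press from its gun end.
; Each Tick adds forward-plus-strafe movement input, then line-traces along the ship's up axis scaled by RaycastLength.
; The hit normal drives root pitch and roll while preserving yaw, and a hit snaps the root to a fixed height along that normal.
; Visual banking and camera-follow logic are disconnected.
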(event EventTick
  (params (DeltaSeconds :type Float%20%28single-precision%29))
  (bind (_startposition _endposition) (CallFunction|RaycastDown))
  ;[0.1887 0.7885 1] Movement
  (LogicMovement|MoveLogicHorizontal DeltaSeconds)
  (bind (_outhit _returnvalue) (Collision|LineTraceByChannel _startposition _endposition "TraceTypeQuery4" true 0 "ForOneFrame"))
  (LogicMovement|RotateLogicbyRaycast (.ImpactNormal (Collision|BreakHitResult _outhit)) DeltaSeconds)
  (if _returnvalue
    (LogicMovement|SetLogicHeight (.ImpactPoint (Collision|BreakHitResult _outhit)) (.ImpactNormal (Collision|BreakHitResult _outhit)))))

(event Input|ActionEvents|InputActionShoot
  (params (Key :type Key%20Structure :default "None"))
  ;[1 0.4495 0.1962] Shooting
  (:Pressed
    (if (not (Variables|Default|GetIsShooting))
      (Variables|Default|SetIsShooting true)
      (Game|SpawnActorfromClass "/Game/Blueprints/BP_StandardBullet.BP_StandardBullet_C" (Transformation|GetWorldTransform (Variables|/Game/Blueprints/BP_PlayerShip_visuals.BP_PlayerShip_visuals_C|GetGunEnd (Variables|Default|GetVisualsReference))) "Undefined" 0 0)))
  (:Released
    (if (Variables|Default|GetIsShooting)
      (Variables|Default|SetIsShooting false))))

(event Input|AxisEvents|InputAxisPlayerRotateRight
  (params (AxisValue :type Float%20%28single-precision%29))
  (Variables|Default|SetMove%20Right%20Axis AxisValue))

(fn ConstructionScript)

(fn MoveLogicHorizontal
  (params (Axis%20Value :type Float%20%28double-precision%29))
  (Pawn|Input|AddMovementInput (+ (* (Transformation|GetActorRightVector) (Variables|Default|GetMove%20Right%20Axis)) (Transformation|GetActorForwardVector)) (* Axis%20Value (Variables|Horizontal|GetHorizontal%20Current%20Speed)) false))

(fn RotateShip
  (params (Axis%20Value :type Float%20%28double-precision%29)))

(fn MoveLogicForward
  (Pawn|Input|AddMovementInput (Transformation|GetActorForwardVector) 1.0 true))

(fn RotateLogicbyRaycast
  (params (Normal :type Vector%20%28by%20ref%29) (DeltaTime :type Float%20%28single-precision%29))
  (bind _root (Variables|Default|GetRoot))
  (bind _returnvalue (Transformation|GetWorldRotation _root))
  (Transformation|SetWorldRotation _root (Math|Interpolation|RInterpTo _returnvalue (Math|Rotator|MakeRotator (.Roll (Math|Rotator|BreakRotator (Math|Rotator|MakeRotfromXZ (Math|Vector|GetForwardVector _root) Normal))) (.Pitch (Math|Rotator|BreakRotator (Class|KismetMathLibrary|MakeRotfromYZ (Math|Vector|GetRightVector _root) Normal))) (.Yaw (Math|Rotator|BreakRotator _returnvalue))) DeltaTime 0.0) false false))

(fn RaycastDown
  (bind _root (Variables|Default|GetRoot))
  (bind _returnvalue (Transformation|GetWorldLocation _root))
  (return _returnvalue (+ _returnvalue (* (Math|Vector|GetUpVector (Transformation|GetWorldRotation _root)) (Variables|Default|GetRaycast%20Length)))))

(fn SetLogicHeight
  (params (Impact%20Point :type Vector) (Impact%20Normal :type Vector))
  (Transformation|SetWorldLocation (Variables|Default|GetRoot) (+ Impact%20Point (* (Math|Vector|Normalize Impact%20Normal) 2e+02)) false false))