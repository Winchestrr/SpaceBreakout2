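; BP_StandardBullet is a bullet actor that fires a visibility line trace every Tick.
; RaycastDown supplies the trace endpoints, running from the root component's location along its up vector scaled by RaycastLength.
; The trace result is not used, and the graphs contain no movement or damage logic.
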(event EventBeginPlay)

(event Collision|EventActorBeginOverlap
  (params (OtherActor :type Actor%20Object%20Reference)))

(event EventTick
  (params (DeltaSeconds :type Float%20%28single-precision%29))
  (bind (_start_position _end_posititon) (CallFunction|RaycastDown))
  (Collision|LineTraceByChannel _start_position _end_posititon "TraceTypeQuery1" false 0 "None" true "(R=0.000000,G=0.678845,B=1.000000,A=1.000000)"))

(fn ConstructionScript)

(fn RaycastDown
  (bind _defaultsceneroot (Variables|Default|GetDefaultSceneRoot))
  (bind _returnvalue (Transformation|GetWorldLocation _defaultsceneroot))
  (return _returnvalue (+ _returnvalue (* (Math|Vector|GetUpVector (Transformation|GetWorldRotation _defaultsceneroot)) (Variables|Default|GetRaycast%20Length)))))