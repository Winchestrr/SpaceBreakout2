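; BP_PlayerShip_visuals is the visual half of the player ship, smoothly trailing a separate PlayerLogic actor.
; Each Tick, GetDesiredMeshLocation lerps from the current transform toward PlayerLogic's rotation and offset location, then applies it to Root.
; The lerp alphas are fixed per frame, without delta-time scaling.
; Camera-follow and downward-trace helpers exist, but their event-graph logic is disconnected and never runs.
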(event EventTick
  (params (DeltaSeconds :type Float%20%28single-precision%29))
  (bind (_player_location _player_rotation) (CallFunction|GetDesiredMeshLocation))
  (Transformation|SetWorldRotation (Variables|Default|GetRoot) _player_rotation false false)
  (Transformation|SetWorldLocation (Variables|Default|GetRoot) _player_location false false))

(fn ConstructionScript)

(fn GetDesiredMeshLocation
  (bind _playerlogic (Variables|Default|GetPlayerLogic))
  (bind _returnvalue (Transformation|GetActorLocation _playerlogic))
  (return (Math|Vector|Lerp(Vector) (Transformation|GetActorLocation) (Math|Vector|MakeVector (+ (.x _returnvalue) (Variables|Default|GetMesh%20X%20Offset)) (.y _returnvalue) (+ (Variables|Default|GetMesh%20Z%20Offset) (.z _returnvalue))) (Variables|Default|GetMesh%20Location%20Lerp%20Speed)) (Math|Rotator|Lerp(Rotator) (Transformation|GetActorRotation) (Transformation|GetActorRotation _playerlogic) (Variables|Default|GetMesh%20Rotation%20Lerp%20Speed))))

(fn GetDesiredCameraLocation
  (bind _playerlogic (Variables|Default|GetPlayerLogic))
  (bind _returnvalue (Transformation|GetActorLocation _playerlogic))
  (return (Math|Vector|MakeVector (+ (.x _returnvalue) (Variables|Default|GetCamera%20X%20Offset)) (.y _returnvalue) (.z _returnvalue)) (Transformation|GetActorRotation _playerlogic)))

(fn RaycastDown
  (bind _root (Variables|Default|GetRoot))
  (bind _returnvalue (Transformation|GetWorldLocation _root))
  (return _returnvalue (+ _returnvalue (* (Math|Vector|GetUpVector (Transformation|GetWorldRotation _root)) -3e+03))))