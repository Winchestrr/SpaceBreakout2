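; A timed power-up pickup that adds one to a BP_PlayerShip_visuals ship's NumberOfBullets while active.
; On overlap with that ship, it increments the count, hides its mesh and turns off collider overlap events.
; A parallel Sequence branch, which runs on any overlap even if the cast fails, waits PowerUpTime, prints a message, decrements the count and destroys the pickup.
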(event OnComponentBeginOverlap(Collider)
  (params (OverlappedComponent :type Primitive%20Component%20Object%20Reference) (OtherActor :type Actor%20Object%20Reference) (OtherComp :type Primitive%20Component%20Object%20Reference) (OtherBodyIndex :type Integer) (bFromSweep :type Boolean) (SweepResult :type Hit%20Result%20Structure%20%28by%20ref%29))
  (Utilities|FlowControl|Sequence
    (:then_0
      (bind _asbp_player_ship_visuals (Utilities|Casting|CastToBP_PlayerShip_visuals OtherActor))
      (Math|Integer|IncrementInt (Variables|/Game/Blueprints/Player/BP_PlayerShip_visuals.BP_PlayerShip_visuals_C|GetNumber%20Of%20Bullets _asbp_player_ship_visuals)
        (:%20%20
          (Rendering|SetVisibility (Variables|Default|GetMesh) false false)
          (Variables|/Script/Engine.PrimitiveComponent|SetbGenerateOverlapEvents (Variables|Default|GetCollider) false))))
    (:then_1
      (Utilities|FlowControl|Delay (Variables|Default|GetPower%20Up%20Time))
      (Development|PrintString "pwup complete")
      (Math|Integer|DecrementInt (Variables|/Game/Blueprints/Player/BP_PlayerShip_visuals.BP_PlayerShip_visuals_C|GetNumber%20Of%20Bullets _asbp_player_ship_visuals)
        (:%20%20
          (Actor|DestroyActor))))))

(fn ConstructionScript)