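; Arena gate actor that stays sealed by a force field until enough smart enemies or buttons are destroyed.
; Both destruction events increment one shared counter, and exactly half the threshold switches the Wwise enemy music to its second state.
; At the threshold it queues a gate-stop voice line on the player ship, posts the arena stop audio event, and destroys the force field and game-over trigger components.
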(event Custom|Smart%20Enemy%20Destroyed
  (bind _forcefield (Variables|Default|GetForceField))
  (bind _smart_enemies_destroyed_to_open (Variables|Default|GetSmart%20Enemies%20Destroyed%20To%20Open))
  (bind _result (Math|Integer|IncrementInt (Variables|Default|GetSmart%20Enemies%20Destroyed))
    (:%20%20
      (if (>= _result _smart_enemies_destroyed_to_open)
        (Utilities|IsValid _forcefield
          (:Is%20Valid
            (bind _returnvalue (Actor|GetActorOfClass "/Game/Blueprints/Player/BP_PlayerShip_logic.BP_PlayerShip_logic_C"))
            (Default|SFXAddtoQue _returnvalue "GoalChange" "Gate_Stop")
            (Class|AkGameplayStatics|PostEvent "/Game/WwiseAudio/Events/Arena/Arena_Stop.Arena_Stop")
            (Components|DestroyComponent _forcefield)
            (Components|DestroyComponent (Variables|Default|GetBP_GameOverTrigger))))
        (elif (== _result (/ _smart_enemies_destroyed_to_open 2))
          (Class|AkGameplayStatics|SetState "/Game/WwiseAudio/States/Enemy_Music_State/Enemy_Music_State-State_2.Enemy_Music_State-State_2"))))))

(event EventBeginPlay)

(event Collision|EventActorBeginOverlap
  (params (OtherActor :type Actor%20Object%20Reference)))

(event EventTick
  (params (DeltaSeconds :type Float%20%28single-precision%29)))

(event EventButtonDestroyed
  (bind _forcefield (Variables|Default|GetForceField))
  (bind _smart_enemies_destroyed_to_open (Variables|Default|GetSmart%20Enemies%20Destroyed%20To%20Open))
  (bind _result (Math|Integer|IncrementInt (Variables|Default|GetSmart%20Enemies%20Destroyed))
    (:%20%20
      (if (>= _result _smart_enemies_destroyed_to_open)
        (Utilities|IsValid _forcefield
          (:Is%20Valid
            (bind _returnvalue (Actor|GetActorOfClass "/Game/Blueprints/Player/BP_PlayerShip_logic.BP_PlayerShip_logic_C"))
            (Default|SFXAddtoQue _returnvalue "GoalChange" "Gate_Stop")
            (Class|AkGameplayStatics|PostEvent "/Game/WwiseAudio/Events/Arena/Arena_Stop.Arena_Stop")
            (Components|DestroyComponent _forcefield)
            (Components|DestroyComponent (Variables|Default|GetBP_GameOverTrigger))))
        (elif (== _result (/ _smart_enemies_destroyed_to_open 2))
          (Class|AkGameplayStatics|SetState "/Game/WwiseAudio/States/Enemy_Music_State/Enemy_Music_State-State_2.Enemy_Music_State-State_2"))))))

(fn ConstructionScript)