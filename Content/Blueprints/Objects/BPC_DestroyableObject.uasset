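; Actor component that gives its owning actor a Life value and destroys that actor when it runs out.
; The Damage event subtracts incoming damage from Life, prints the result and destroys the owner at zero or below.
; The node binding this event to the owner's OnTakeAnyDamage is unconnected and never runs, so the graph does not hook up damage by itself.
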(event Custom|Damage
  (params (DamagedActor :type Actor%20Object%20Reference) (Damage :type Float%20%28single-precision%29) (DamageType :type Damage%20Type%20Object%20Reference) (InstigatedBy :type Controller%20Object%20Reference) (DamageCauser :type Actor%20Object%20Reference))
  (bind _output_get (Variables|Default|SetLife (- (Variables|Default|GetLife) Damage)))
  (Development|PrintString (Utilities|String|ToString(Float) _output_get))
  (if (<= _output_get 0.0)
    (Actor|DestroyActor (Components|GetOwner))))

(event EventBeginPlay)

(event EventTick
  (params (DeltaSeconds :type Float%20%28single-precision%29)))