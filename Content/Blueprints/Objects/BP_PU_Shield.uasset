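; Shield power-up pickup that temporarily protects the player ship when it overlaps the pickup's collider.
; On overlap with BP_PlayerShip_visuals, it shows the shield and moves overlap detection from the ship's collider to the shield collider.
; After PowerUpTime, a looping delay blinks the shield for MaxTickAmount cycles as an expiry warning.
; It then restores the ship's normal collision, hides the shield and destroys itself.
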(event OnComponentBeginOverlap(Collider)
  (params (OverlappedComponent :type Primitive%20Component%20Object%20Reference) (OtherActor :type Actor%20Object%20Reference) (OtherComp :type Primitive%20Component%20Object%20Reference) (OtherBodyIndex :type Integer) (bFromSweep :type Boolean) (SweepResult :type Hit%20Result%20Structure%20%28by%20ref%29))
  (Utilities|FlowControl|Sequence
    (:then_0
      (Variables|Default|SetCurrent%20Ticks 0)
      (bind _asbp_player_ship_visuals (Utilities|Casting|CastToBP_PlayerShip_visuals OtherActor))
      (Variables|Default|SetPlayer%20Visuals _asbp_player_ship_visuals)
      (Rendering|SetVisibility (Variables|/Game/Blueprints/Player/BP_PlayerShip_visuals.BP_PlayerShip_visuals_C|GetShield (Variables|Default|GetPlayer%20Visuals)) true false)
      (Variables|/Script/Engine.PrimitiveComponent|SetbGenerateOverlapEvents (Variables|/Game/Blueprints/Player/BP_PlayerShip_visuals.BP_PlayerShip_visuals_C|GetShield%20Collider (Variables|Default|GetPlayer%20Visuals)) true)
      (Rendering|SetVisibility (Variables|/Game/Blueprints/Player/BP_PlayerShip_visuals.BP_PlayerShip_visuals_C|GetShield%20Collider (Variables|Default|GetPlayer%20Visuals)) true false)
      (Variables|/Script/Engine.PrimitiveComponent|SetbGenerateOverlapEvents (Variables|/Game/Blueprints/Player/BP_PlayerShip_visuals.BP_PlayerShip_visuals_C|GetCollider (Variables|Default|GetPlayer%20Visuals)) false))
    (:then_1
      (Utilities|FlowControl|Delay (Variables|Default|GetPower%20Up%20Time))
      (Rendering|SetVisibility (Variables|/Game/Blueprints/Player/BP_PlayerShip_visuals.BP_PlayerShip_visuals_C|GetShield (Variables|Default|GetPlayer%20Visuals)) false false :!label _label)
      (Utilities|FlowControl|Delay 0.1)
      (Rendering|SetVisibility (Variables|/Game/Blueprints/Player/BP_PlayerShip_visuals.BP_PlayerShip_visuals_C|GetShield (Variables|Default|GetPlayer%20Visuals)) true false)
      (Utilities|FlowControl|Delay 0.1)
      (Math|Integer|IncrementInt (Variables|Default|GetCurrent%20Ticks)
        (:%20%20
          (if (>= (Variables|Default|GetCurrent%20Ticks) (Variables|Default|GetMax%20Tick%20Amount))
            (Development|PrintString "pwup complete")
            (Rendering|SetVisibility (Variables|/Game/Blueprints/Player/BP_PlayerShip_visuals.BP_PlayerShip_visuals_C|GetShield (Variables|Default|GetPlayer%20Visuals)) false false)
            (Variables|/Script/Engine.PrimitiveComponent|SetbGenerateOverlapEvents (Variables|/Game/Blueprints/Player/BP_PlayerShip_visuals.BP_PlayerShip_visuals_C|GetShield%20Collider (Variables|Default|GetPlayer%20Visuals)) false)
            (Rendering|SetVisibility (Variables|/Game/Blueprints/Player/BP_PlayerShip_visuals.BP_PlayerShip_visuals_C|GetShield%20Collider (Variables|Default|GetPlayer%20Visuals)) false false)
            (Variables|/Script/Engine.PrimitiveComponent|SetbGenerateOverlapEvents (Variables|/Game/Blueprints/Player/BP_PlayerShip_visuals.BP_PlayerShip_visuals_C|GetCollider (Variables|Default|GetPlayer%20Visuals)) true)
            (Actor|DestroyActor)
            (else
              (goto _label))))))))

(event EventBeginPlay)

(event Collision|EventActorBeginOverlap
  (params (OtherActor :type Actor%20Object%20Reference)))

(event EventTick
  (params (DeltaSeconds :type Float%20%28single-precision%29)))

(fn ConstructionScript)