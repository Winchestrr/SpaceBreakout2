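; BP_EnemyEnterSpline is a spline actor that brings a BP_BigEnemy into the scene along an entrance path.
; StartEntering spawns the enemy at the first spline point, assigns its configured type, and disables its floating component and shooting.
; A Timeline drives its location and rotation along the spline's length, then re-enables floating and starts shooting when finished.
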(event Custom|Start%20Entering
  (Development|PrintString "spline activated")
  (bind _returnvalue (Game|SpawnActorfromClass "/Game/Blueprints/Enemies/BP_BigEnemy.BP_BigEnemy_C" (Math|Transform|MakeTransform (Spline|GetLocationatSplinePoint (Variables|Default|GetSpline) 0 "World") "0, 0, 0" "1.000000,1.000000,1.000000") "Undefined" 0 0))
  (Variables|Default|SetEnemy _returnvalue)
  (Variables|/Game/Blueprints/Objects/BPC_FloatingObject.BPC_FloatingObject_C|SetIs%20Component%20Active (Variables|/Game/Blueprints/Enemies/BP_BigEnemy.BP_BigEnemy_C|GetBPC_FloatingObject (Variables|Default|GetEnemy)) false)
  (Variables|/Game/Blueprints/Enemies/BP_BigEnemy.BP_BigEnemy_C|SetCan%20Shoot (Variables|Default|GetEnemy) false)
  (Variables|Default|SetIs%20Moving true)
  (Variables|/Game/Blueprints/Enemies/BP_BigEnemy.BP_BigEnemy_C|SetEnemy%20Type (Variables|Default|GetEnemy) (Variables|Default|GetSpawn%20Enemy%20Type))
  (bind _float_track (Timeline|Timeline Play)
    (:Update
      (Transformation|SetActorLocationAndRotation (Variables|Default|GetEnemy) (Spline|GetLocationatDistanceAlongSpline (Variables|Default|GetSpline) (Math|Float|Lerp 0.0 (Spline|GetSplineLength (Variables|Default|GetSpline)) _float_track) "World") (Spline|GetRotationatDistanceAlongSpline (Variables|Default|GetSpline) (Math|Float|Lerp 0.0 (Spline|GetSplineLength (Variables|Default|GetSpline)) _float_track) "World")))
    (:Finished
      (Variables|/Game/Blueprints/Objects/BPC_FloatingObject.BPC_FloatingObject_C|SetIs%20Component%20Active (Variables|/Game/Blueprints/Enemies/BP_BigEnemy.BP_BigEnemy_C|GetBPC_FloatingObject (Variables|Default|GetEnemy)) true)
      (Variables|Default|SetIs%20Moving false)
      (Variables|/Game/Blueprints/Enemies/BP_BigEnemy.BP_BigEnemy_C|SetCan%20Shoot (Variables|Default|GetEnemy) true)
      (Default|StartShooting (Variables|Default|GetEnemy)))))

(event EventTick
  (params (DeltaSeconds :type Float%20%28single-precision%29)))

(fn ConstructionScript)