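; BP_Button is a shootable button that breaks when hit by a Bullet-tagged actor and notifies its linked Gate.
; On the first hit, Collider overlap sets a destroyed flag, spawns an explosion particle, swaps the intact mesh for a damaged one and sends the destroyed message to the Gate.
; The bullet is then destroyed, and the flag makes later overlaps do nothing.
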(event OnComponentBeginOverlap(Collider)
  (params (OverlappedComponent :type Primitive%20Component%20Object%20Reference) (OtherActor :type Actor%20Object%20Reference) (OtherComp :type Primitive%20Component%20Object%20Reference) (OtherBodyIndex :type Integer) (bFromSweep :type Boolean) (SweepResult :type Hit%20Result%20Structure%20%28by%20ref%29))
  (if (not (Variables|Default|GetIs%20Destroyed))
    (if (Actor|ActorHasTag OtherActor "Bullet")
      (Utilities|FlowControl|Sequence
        (:then_0
          (Variables|Default|SetIs%20Destroyed true)
          (Game|SpawnActorfromClass "/Game/Realistic_Starter_VFX_Pack_Vol2/Blueprints/BP_ExplosionParticle.BP_ExplosionParticle_C" (Transformation|GetWorldTransform (Variables|Default|GetParticleSpawn)) "AlwaysSpawn" 0 0)
          (Rendering|SetVisibility (Variables|Default|GetMesh) false false)
          (Rendering|SetVisibility (Variables|Default|GetDamagedMesh) true false)
          (Class|BPIButtonGateConnect|ButtonDestroyed(Message) (Variables|Default|GetGate)))
        (:then_1
          (Actor|DestroyActor OtherActor))))))

(event EventBeginPlay
  (Rendering|SetVisibility (Variables|Default|GetMesh) true false)
  (Rendering|SetVisibility (Variables|Default|GetDamagedMesh) false false))

(event Collision|EventActorBeginOverlap
  (params (OtherActor :type Actor%20Object%20Reference)))

(event EventTick
  (params (DeltaSeconds :type Float%20%28single-precision%29)))

(fn ConstructionScript)