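; Actor component that makes its owner glide over surfaces at a fixed hover height, then fall and be destroyed when the surface ends.
; While IsFalling is true, it moves the owner forward and sideways, traces along its up axis and snaps it off the hit point.
; Rotation eases toward the surface normal, optionally taking yaw from the nearest BP_Spline point.
; On a missed trace, non-bullets clear IsFalling, drop, and are destroyed after DestroyTime.
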(event EventBeginPlay
  (Variables|Default|SetOwner (Components|GetOwner))
  (bind _returnvalue (Actor|GetActorOfClass "/Game/Blueprints/BP_Spline.BP_Spline_C"))
  (Variables|Default|SetSpline _returnvalue))

(event EventTick
  (params (DeltaSeconds :type Float%20%28single-precision%29))
  (bind _spline (Variables|Default|GetSpline))
  (bind _owner (Variables|Default|GetOwner))
  (bind _owner_2 (Variables|Default|GetOwner))
  (bind _owner_3 (Variables|Default|GetOwner))
  (bind _owner_4 (Variables|Default|GetOwner))
  (bind _spline_2 (Variables|/Game/Blueprints/BP_Spline.BP_Spline_C|GetSpline _spline))
  (bind _rootcomponent (Variables|/Script/Engine.Actor|GetRootComponent _owner))
  (bind _rootcomponent_2 (Variables|/Script/Engine.Actor|GetRootComponent _owner_3))
  (bind _rootcomponent_3 (Variables|/Script/Engine.Actor|GetRootComponent _owner_4))
  (bind _returnvalue (Transformation|GetWorldLocation _rootcomponent))
  (bind _returnvalue_2 (Transformation|GetWorldRotation _rootcomponent_3))
  (Variables|Default|SetDelta%20Seconds DeltaSeconds)
  (if (Variables|Default|GetIs%20Falling)
    (Transformation|SetActorLocation (Variables|Default|GetOwner) (+ (Transformation|GetActorLocation _owner_2) (* (Transformation|GetActorForwardVector _owner_2) (Variables|Default|GetSpeed%20Forward) (Variables|Default|GetDelta%20Seconds)) (* (Transformation|GetActorRightVector _owner_2) (Variables|Default|GetSpeed%20Right) (Variables|Default|GetDelta%20Seconds))) false false)
    (Utilities|IsValid (Components|GetOwner)
      (:Is%20Valid
        (bind (_outhit _returnvalue_3) (Collision|LineTraceByChannel _returnvalue (+ _returnvalue (* (Math|Vector|GetUpVector (Transformation|GetWorldRotation (Variables|/Script/Engine.Actor|GetRootComponent _owner))) (Variables|Default|GetRaycast%20Length))) "TraceTypeQuery3" true 0 "None" false))
        (if _returnvalue_3
          (if (Variables|Default|GetIs%20Rotated%20By%20Spline)
            (Transformation|SetWorldRotation _rootcomponent_3 (Math|Interpolation|RInterpTo _returnvalue_2 (Math|Rotator|MakeRotator (.Roll (Math|Rotator|BreakRotator (Math|Rotator|MakeRotfromXZ (Math|Vector|GetForwardVector _rootcomponent_3) (.Normal (Collision|BreakHitResult _outhit))))) (.Pitch (Math|Rotator|BreakRotator (Class|KismetMathLibrary|MakeRotfromYZ (Math|Vector|GetRightVector _rootcomponent_3) (.Normal (Collision|BreakHitResult _outhit))))) (.yaw (Class|SplineComponent|GetRotationatSplineInputKey _spline_2 (Class|SplineComponent|FindInputKeyClosesttoWorldLocation _spline_2 (Transformation|GetWorldLocation _rootcomponent_3)) "World"))) (Variables|Default|GetDelta%20Seconds) 0.0) false false)
            (else
              (Transformation|SetWorldRotation _rootcomponent_3 (Math|Interpolation|RInterpTo _returnvalue_2 (Math|Rotator|MakeRotator (.Roll (Math|Rotator|BreakRotator (Math|Rotator|MakeRotfromXZ (Math|Vector|GetForwardVector _rootcomponent_3) (.Normal (Collision|BreakHitResult _outhit))))) (.Pitch (Math|Rotator|BreakRotator (Class|KismetMathLibrary|MakeRotfromYZ (Math|Vector|GetRightVector _rootcomponent_3) (.Normal (Collision|BreakHitResult _outhit))))) (.Yaw (Math|Rotator|BreakRotator _returnvalue_2))) (Variables|Default|GetDelta%20Seconds) 0.0) false false)))
          (Transformation|SetActorLocation (Variables|Default|GetOwner) (+ (.ImpactPoint (Collision|BreakHitResult _outhit)) (* (Math|Vector|Normalize (.ImpactNormal (Collision|BreakHitResult _outhit))) 2e+02)) false false)
          (elif (not (Variables|Default|GetIs%20Bullet))
            (Variables|Default|SetIs%20Falling false)
            (Utilities|FlowControl|Delay (Variables|Default|GetDestroy%20Time))
            (Actor|DestroyActor (Variables|Default|GetOwner))))))
    (else
      (Transformation|SetWorldLocation _rootcomponent_2 (+ (Transformation|GetWorldLocation _rootcomponent_2) (* (Math|Vector|GetUpVector _rootcomponent_2) (Variables|Default|GetDelta%20Seconds) (Variables|Default|GetFall%20Speed%20Down) -1.0) (* (Math|Vector|GetForwardVector _rootcomponent_2) (Variables|Default|GetDelta%20Seconds) (Variables|Default|GetFall%20Speed%20Forward))) false false))))