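; BP_PU_DamageUp_2 is a timed damage power-up pickup for the player ship.
; On collider overlap, it casts to BP_PlayerShip_visuals, saves the Damage on its LogicReference and multiplies it by PowerUpValue.
; It then hides the mesh and stops overlap events, keeping the actor alive as the timer.
; A second sequence branch waits PowerUpTime, restores the saved damage and destroys the actor.
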(event OnComponentBeginOverlap(Collider)
  (params (OverlappedComponent :type Primitive%20Component%20Object%20Reference) (OtherActor :type Actor%20Object%20Reference) (OtherComp :type Primitive%20Component%20Object%20Reference) (OtherBodyIndex :type Integer) (bFromSweep :type Boolean) (SweepResult :type Hit%20Result%20Structure%20%28by%20ref%29))
  (Utilities|FlowControl|Sequence
    (:then_0
      (bind _asbp_player_ship_visuals (Utilities|Casting|CastToBP_PlayerShip_visuals OtherActor)
        (:then
          (bind _output_get (Variables|Default|SetOld%20Damage%20Value (Variables|/Game/Blueprints/Player/BP_PlayerShip_logic.BP_PlayerShip_logic_C|GetDamage (Variables|/Game/Blueprints/Player/BP_PlayerShip_visuals.BP_PlayerShip_visuals_C|GetLogic%20Reference _asbp_player_ship_visuals))))
          (Variables|/Game/Blueprints/Player/BP_PlayerShip_logic.BP_PlayerShip_logic_C|SetDamage (Variables|/Game/Blueprints/Player/BP_PlayerShip_visuals.BP_PlayerShip_visuals_C|GetLogic%20Reference _asbp_player_ship_visuals) (* _output_get (Variables|Default|GetPower%20Up%20Value))))
        (:CastFailed
          _))
      (Rendering|SetVisibility (Variables|Default|GetMesh) false false)
      (Variables|/Script/Engine.PrimitiveComponent|SetbGenerateOverlapEvents (Variables|Default|GetCollider) false))
    (:then_1
      (Utilities|FlowControl|Delay (Variables|Default|GetPower%20Up%20Time))
      (Development|PrintString "pwup complete")
      (Variables|/Game/Blueprints/Player/BP_PlayerShip_logic.BP_PlayerShip_logic_C|SetDamage (Variables|/Game/Blueprints/Player/BP_PlayerShip_visuals.BP_PlayerShip_visuals_C|GetLogic%20Reference _asbp_player_ship_visuals) (Variables|Default|GetOld%20Damage%20Value))
      (Actor|DestroyActor))))

(event EventBeginPlay)

(event Collision|EventActorBeginOverlap
  (params (OtherActor :type Actor%20Object%20Reference)))

(event EventTick
  (params (DeltaSeconds :type Float%20%28single-precision%29)))

(fn ConstructionScript)