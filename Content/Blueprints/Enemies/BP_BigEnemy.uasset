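; BP_BigEnemy is a shooting enemy that awards points to the player ship when killed.
; From BeginPlay, a Delay-driven loop traces forward from the gun, firing bullets with random odds.
; It fires faster when the trace hits the player and re-randomizes its delay when blocked by another enemy.
; DealDamage decrements health; on death it hides, explodes, adds points and destroys itself after a delay.
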(event EventBeginPlay
  (bind (_start _end) (CallFunction|RaycastForward))
  (Utilities|FlowControl|Delay (Math|Random|RandomFloatinRange 0.0 (Variables|Default|GetTime%20Between%20Shots)) :!label _label)
  (bind (_outhit _returnvalue) (Collision|LineTraceByChannel _start _end "TraceTypeQuery4" false 0 "ForOneFrame" :!label _label_2))
  (if (and (Variables|Default|GetCan%20Shoot) (not (Variables|Default|GetIs%20Dead)))
    (if _returnvalue
      (Variables|Default|SetCurrent%20TBS (/ (Variables|Default|GetTime%20Between%20Shots) 4.0))
      (if (Actor|ActorHasTag (.HitActor (Collision|BreakHitResult _outhit)) "Player")
        ;[1 1 1] Shoot
        (Utilities|FlowControl|Sequence :!label _label_3
          (:then_0
            (Variables|Default|SetCan%20Shoot false)
            ;;[1 0.9265 0.2541] Shoot probability
            (if (<= (Math|Random|RandomFloatinRange 0.0 1.0) 0.7)
              (Game|SpawnActorfromClass "/Game/Blueprints/Weapons/BP_EnemyBullet.BP_EnemyBullet_C" (Transformation|GetWorldTransform (Variables|Default|GetGun%20End)) "Undefined" 0 0)))
          (:then_1
            (Utilities|FlowControl|Delay (Variables|Default|GetCurrent%20TBS))
            (Variables|Default|SetCan%20Shoot true)
            (goto _label_2)))
        (elif (Actor|ActorHasTag (.HitActor (Collision|BreakHitResult _outhit)) "Enemy")
          (goto _label)))
      (else
        (Variables|Default|SetCurrent%20TBS (Variables|Default|GetTime%20Between%20Shots))
        (goto _label_3)))))

(event EventDealDamage
  (params (NewDamage :type Float%20%28double-precision%29) (Hit%20Component :type Actor%20Component%20Object%20Reference))
  (Math|Float|DecrementFloat (Variables|Default|GetHealth)
    (:%20%20
      (if (<= (Variables|Default|GetHealth) 0.0)
        (Utilities|FlowControl|Sequence
          (:then_0
            (Variables|Default|SetIs%20Dead true)
            (Variables|/Script/Engine.PrimitiveComponent|SetbGenerateOverlapEvents (Variables|Default|GetBox) false)
            (Rendering|SetVisibility (Variables|Default|GetMesh) false false)
            (Game|SpawnActorfromClass "/Game/Realistic_Starter_VFX_Pack_Vol2/Blueprints/BP_ExplosionParticle.BP_ExplosionParticle_C" (Transformation|GetWorldTransform (Variables|Default|GetDefaultSceneRoot)) "Undefined" 0 0))
          (:then_1
            (bind _returnvalue (Actor|GetActorOfClass "/Game/Blueprints/Player/BP_PlayerShip_logic.BP_PlayerShip_logic_C"))
            (Variables|/Game/Blueprints/Player/BP_PlayerShip_logic.BP_PlayerShip_logic_C|SetPoints _returnvalue (+ (Variables|/Game/Blueprints/Player/BP_PlayerShip_logic.BP_PlayerShip_logic_C|GetPoints _returnvalue) (Variables|Default|GetPoint%20Value))))
          (:then_2
            (Utilities|FlowControl|Delay 3.0)
            (Actor|DestroyActor)))))))

(fn ConstructionScript)

(fn RaycastForward
  (bind _gun_end (Variables|Default|GetGun%20End))
  (bind _returnvalue (Transformation|GetWorldLocation _gun_end))
  (return _returnvalue (+ _returnvalue (* (Math|Vector|GetForwardVector _gun_end) (Variables|Default|GetShooting%20Range)))))