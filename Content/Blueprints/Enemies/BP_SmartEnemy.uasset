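; Enemy ship that turns its gun toward a nearby player, fires and dodges sideways, awarding points when destroyed.
; A delayed trace loop fires probabilistically, faster with the player in line and holding fire behind other enemies.
; Side collider overlaps randomly trigger brief lateral bursts through the floating-object component.
; Player bullets reduce health; death spawns an explosion, notifies ArenaGate and destroys the actor after a delay.
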(event OnComponentBeginOverlap(PlayerSearchCollider)
  (params (OverlappedComponent :type Primitive%20Component%20Object%20Reference) (OtherActor :type Actor%20Object%20Reference) (OtherComp :type Primitive%20Component%20Object%20Reference) (OtherBodyIndex :type Integer) (bFromSweep :type Boolean) (SweepResult :type Hit%20Result%20Structure%20%28by%20ref%29))
  (if (Actor|ActorHasTag OtherActor "Player")
    (Variables|Default|SetOther%20Actor OtherActor)
    (Variables|Default|SetIs%20Player%20In%20Range true)))

(event OnComponentEndOverlap(PlayerSearchCollider)
  (params (OverlappedComponent :type Primitive%20Component%20Object%20Reference) (OtherActor :type Actor%20Object%20Reference) (OtherComp :type Primitive%20Component%20Object%20Reference) (OtherBodyIndex :type Integer))
  (if (Actor|ActorHasTag OtherActor "Player")
    (Variables|Default|SetIs%20Player%20In%20Range false)))

(event OnComponentBeginOverlap(Collider)
  (params (OverlappedComponent :type Primitive%20Component%20Object%20Reference) (OtherActor :type Actor%20Object%20Reference) (OtherComp :type Primitive%20Component%20Object%20Reference) (OtherBodyIndex :type Integer) (bFromSweep :type Boolean) (SweepResult :type Hit%20Result%20Structure%20%28by%20ref%29))
  (bind _asbp_standard_bullet (Utilities|Casting|CastToBP_StandardBullet OtherActor))
  (bind _returnvalue (Actor|GetActorOfClass "/Game/Blueprints/Player/BP_PlayerShip_logic.BP_PlayerShip_logic_C"))
  (Variables|Default|SetHealth (- (Variables|Default|GetHealth) (Variables|/Game/Blueprints/Player/BP_PlayerShip_logic.BP_PlayerShip_logic_C|GetDamage _returnvalue)))
  (if (<= (Variables|Default|GetHealth) 0.0)
    (Utilities|FlowControl|Sequence
      (:then_0
        (Variables|Default|SetIs%20Dead true)
        (Variables|/Script/Engine.PrimitiveComponent|SetbGenerateOverlapEvents (Variables|Default|GetCollider) false)
        (Rendering|SetVisibility (Variables|Default|GetMesh) false false)
        (Variables|/Script/Engine.PrimitiveComponent|SetbGenerateOverlapEvents (Variables|Default|GetPlayer%20Search%20Collider) false)
        (Variables|/Script/Engine.PrimitiveComponent|SetbGenerateOverlapEvents (Variables|Default|GetBullet%20Search%20Collider%20Right) false)
        (Variables|/Script/Engine.PrimitiveComponent|SetbGenerateOverlapEvents (Variables|Default|GetBullet%20Search%20Collider%20Left) false)
        (Game|SpawnActorfromClass "/Game/Realistic_Starter_VFX_Pack_Vol2/Blueprints/BP_ExplosionParticle.BP_ExplosionParticle_C" (Transformation|GetWorldTransform (Variables|Default|GetDefaultSceneRoot)) "Undefined" 0 0))
      (:then_1
        (bind _returnvalue_2 (Actor|GetActorOfClass "/Game/Blueprints/Player/BP_PlayerShip_logic.BP_PlayerShip_logic_C"))
        (Variables|/Game/Blueprints/Player/BP_PlayerShip_logic.BP_PlayerShip_logic_C|SetPoints _returnvalue_2 (+ (Variables|/Game/Blueprints/Player/BP_PlayerShip_logic.BP_PlayerShip_logic_C|GetPoints _returnvalue_2) (Variables|Default|GetPoint%20Value))))
      (:then_2
        (Default|SmartEnemyDestroyed (Variables|Default|GetArena%20Gate)))
      (:then_3
        (Utilities|FlowControl|Delay 3.0)
        (Actor|DestroyActor)))))

(event OnComponentBeginOverlap(BulletSearchColliderRight)
  (params (OverlappedComponent :type Primitive%20Component%20Object%20Reference) (OtherActor :type Actor%20Object%20Reference) (OtherComp :type Primitive%20Component%20Object%20Reference) (OtherBodyIndex :type Integer) (bFromSweep :type Boolean) (SweepResult :type Hit%20Result%20Structure%20%28by%20ref%29))
  ;[0.3846 0.9701 1] Random dodge chance
  (if (<= (Variables|Default|GetHit%20Chance) (Math|Random|RandomFloatinRange 0.0 1.0))
    (Utilities|Dodge 4e+03)))

(event OnComponentEndOverlap(BulletSearchColliderRight)
  (params (OverlappedComponent :type Primitive%20Component%20Object%20Reference) (OtherActor :type Actor%20Object%20Reference) (OtherComp :type Primitive%20Component%20Object%20Reference) (OtherBodyIndex :type Integer))
  ;[1 1 1] Dodge Right
)

(event OnComponentBeginOverlap(BulletSearchColliderLeft)
  (params (OverlappedComponent :type Primitive%20Component%20Object%20Reference) (OtherActor :type Actor%20Object%20Reference) (OtherComp :type Primitive%20Component%20Object%20Reference) (OtherBodyIndex :type Integer) (bFromSweep :type Boolean) (SweepResult :type Hit%20Result%20Structure%20%28by%20ref%29))
  ;[0.3846 0.9701 1] Random dodge chance
  (if (<= (Variables|Default|GetHit%20Chance) (Math|Random|RandomFloatinRange 0.0 1.0))
    (Utilities|Dodge -4e+03)))

(event OnComponentEndOverlap(BulletSearchColliderLeft)
  (params (OverlappedComponent :type Primitive%20Component%20Object%20Reference) (OtherActor :type Actor%20Object%20Reference) (OtherComp :type Primitive%20Component%20Object%20Reference) (OtherBodyIndex :type Integer))
  ;[1 1 1] Dodge Left
)

(event Custom|Start%20Shooting
  (bind (_start _end) (CallFunction|RaycastForward))
  (bind _gun_end (Variables|Default|GetGun%20End))
  (bind _returnvalue (Transformation|GetWorldTransform _gun_end))
  (Utilities|FlowControl|Delay (Math|Random|RandomFloatinRange 0.0 (Variables|Default|GetTime%20Between%20Shots)) :!label _label)
  (bind (_outhit _returnvalue_2) (Collision|LineTraceByChannel _start _end "TraceTypeQuery4" false 0 "ForOneFrame" :!label _label_2))
  (if (and (Variables|Default|GetCan%20Shoot) (not (Variables|Default|GetIs%20Dead)))
    (if _returnvalue_2
      (Variables|Default|SetCurrent%20TBS (/ (Variables|Default|GetTime%20Between%20Shots) 4.0))
      (if (Actor|ActorHasTag (.HitActor (Collision|BreakHitResult _outhit)) "Player")
        ;[1 1 1] Shoot
        (Utilities|FlowControl|Sequence :!label _label_3
          (:then_0
            (Variables|Default|SetCan%20Shoot false)
            ;;[1 0.9265 0.2541] Shoot probability
            (if (<= (Math|Random|RandomFloatinRange 0.0 1.0) 0.7)
              (Game|SpawnActorfromClass "/Game/Blueprints/Weapons/BP_SmartEnemyBullet.BP_SmartEnemyBullet_C" (Math|Transform|MakeTransform (.location _returnvalue) (.rotation _returnvalue) "1.000000,1.000000,1.000000") "Undefined" self 0)))
          (:then_1
            (Utilities|FlowControl|Delay (Variables|Default|GetCurrent%20TBS))
            (Variables|Default|SetCan%20Shoot true)
            (goto _label_2)))
        (elif (Actor|ActorHasTag (.HitActor (Collision|BreakHitResult _outhit)) "Enemy")
          (goto _label)))
      (else
        (Variables|Default|SetCurrent%20TBS (Variables|Default|GetTime%20Between%20Shots))
        (goto _label_3)))))

(event Custom|CustomEvent
  (params (NewDamage :type Float%20%28double-precision%29) (Hit%20Component :type Actor%20Component%20Object%20Reference) (Hit%20Actor :type Actor%20Object%20Reference)))

(event EventBeginPlay
  (bind (_start _end) (CallFunction|RaycastForward))
  (bind _gun_end (Variables|Default|GetGun%20End))
  (bind _returnvalue (Transformation|GetWorldTransform _gun_end))
  (Utilities|FlowControl|Delay (Math|Random|RandomFloatinRange 0.0 (Variables|Default|GetTime%20Between%20Shots)) :!label _label)
  (bind (_outhit _returnvalue_2) (Collision|LineTraceByChannel _start _end "TraceTypeQuery4" false 0 "ForOneFrame" :!label _label_2))
  (if (and (Variables|Default|GetCan%20Shoot) (not (Variables|Default|GetIs%20Dead)))
    (if _returnvalue_2
      (Variables|Default|SetCurrent%20TBS (/ (Variables|Default|GetTime%20Between%20Shots) 4.0))
      (if (Actor|ActorHasTag (.HitActor (Collision|BreakHitResult _outhit)) "Player")
        ;[1 1 1] Shoot
        (Utilities|FlowControl|Sequence :!label _label_3
          (:then_0
            (Variables|Default|SetCan%20Shoot false)
            ;;[1 0.9265 0.2541] Shoot probability
            (if (<= (Math|Random|RandomFloatinRange 0.0 1.0) 0.7)
              (Game|SpawnActorfromClass "/Game/Blueprints/Weapons/BP_SmartEnemyBullet.BP_SmartEnemyBullet_C" (Math|Transform|MakeTransform (.location _returnvalue) (.rotation _returnvalue) "1.000000,1.000000,1.000000") "Undefined" self 0)))
          (:then_1
            (Utilities|FlowControl|Delay (Variables|Default|GetCurrent%20TBS))
            (Variables|Default|SetCan%20Shoot true)
            (goto _label_2)))
        (elif (Actor|ActorHasTag (.HitActor (Collision|BreakHitResult _outhit)) "Enemy")
          (goto _label)))
      (else
        (Variables|Default|SetCurrent%20TBS (Variables|Default|GetTime%20Between%20Shots))
        (goto _label_3)))))

(event EventTick
  (params (DeltaSeconds :type Float%20%28single-precision%29))
  (bind _other_actor (Variables|Default|GetOther%20Actor))
  (bind _gun_end (Variables|Default|GetGun%20End))
  (bind _returnvalue (Transformation|GetActorLocation _other_actor))
  (bind _returnvalue_2 (Transformation|GetWorldRotation _gun_end))
  (bind _returnvalue_3 (Transformation|GetWorldLocation _gun_end))
  (bind _returnvalue_4 (Math|Rotator|FindLookatRotation _returnvalue_3 _returnvalue))
  (bind _returnvalue_5 (- (.yaw _returnvalue_4) (.yaw _returnvalue_2)))
  (if (Variables|Default|GetIs%20Player%20In%20Range)
    (if (> (Math|Float|Absolute(Float) _returnvalue_5) 0.1)
      (Transformation|SetWorldRotation (Variables|Default|GetGun%20End) (Math|Rotator|MakeRotator (.roll _returnvalue_2) (.pitch _returnvalue_2) (+ (.yaw _returnvalue_2) (* DeltaSeconds (Math|Float|Sign(Float) _returnvalue_5) (Variables|Default|GetDegreesPerSec)))) false false))))

(fn ConstructionScript)

(fn RaycastForward
  (bind _gun_end (Variables|Default|GetGun%20End))
  (bind _returnvalue (Transformation|GetWorldLocation _gun_end))
  (return _returnvalue (+ _returnvalue (* (Math|Vector|GetForwardVector _gun_end) (Variables|Default|GetShooting%20Range)))))