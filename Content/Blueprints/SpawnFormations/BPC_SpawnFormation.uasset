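; BPC_SpawnFormation is an actor component that spawns a formation of BP_BigEnemy ships laid out by its owner's components.
; On BeginPlay it spawns one enemy at each direct child of the owner's root, with yaw turned 180 degrees and collisions ignored.
; It then disables spline-driven rotation on each enemy's BPCFloatingObject and sets its speed to the player ship's standard forward speed.
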(event EventBeginPlay
  (for _array_element (Components|GetChildrenComponents (Variables|/Script/Engine.Actor|GetRootComponent (Components|GetOwner)) false)
    (bind _returnvalue (Game|SpawnActorfromClass "/Game/Blueprints/BP_BigEnemy.BP_BigEnemy_C" (Math|Transform|MakeTransform (Transformation|GetWorldLocation _array_element) (Math|Rotator|MakeRotator (.roll (Transformation|GetWorldRotation _array_element)) (.pitch (Transformation|GetWorldRotation _array_element)) (+ (.yaw (Transformation|GetWorldRotation _array_element)) 1.8e+02))) "AlwaysSpawn" 0 0))
    (bind _returnvalue_2 (Actor|GetActorOfClass "/Game/Blueprints/Player/BP_PlayerShip_logic.BP_PlayerShip_logic_C"))
    (Variables|/Game/Blueprints/Objects/BPC_FloatingObject.BPC_FloatingObject_C|SetIs%20Rotated%20By%20Spline (Variables|/Game/Blueprints/BP_BigEnemy.BP_BigEnemy_C|GetBPC_FloatingObject _returnvalue) false)
    (Variables|/Game/Blueprints/Objects/BPC_FloatingObject.BPC_FloatingObject_C|SetSpeed (Variables|/Game/Blueprints/BP_BigEnemy.BP_BigEnemy_C|GetBPC_FloatingObject _returnvalue) (Variables|/Game/Blueprints/Player/BP_PlayerShip_logic.BP_PlayerShip_logic_C|GetStandard%20MSpeed%20Forward _returnvalue_2))))