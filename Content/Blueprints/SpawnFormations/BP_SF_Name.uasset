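; Spawn formation trigger that spawns a group of BP_BigEnemy actors when the player ship's visual actor overlaps its Collider.
; Arrow components directly under the root mark the spawn points, with each enemy placed at an arrow's location and yawed 180 degrees from it.
; Each enemy's floating-object component has spline rotation disabled and takes its forward speed from the player logic actor's standard speed.
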(event OnComponentBeginOverlap(Collider)
  (params (OverlappedComponent :type Primitive%20Component%20Object%20Reference) (OtherActor :type Actor%20Object%20Reference) (OtherComp :type Primitive%20Component%20Object%20Reference) (OtherBodyIndex :type Integer) (bFromSweep :type Boolean) (SweepResult :type Hit%20Result%20Structure%20%28by%20ref%29))
  (Utilities|Casting|CastToBP_PlayerShip_visuals OtherActor)
  (for _array_element (Components|GetChildrenComponents (Variables|Default|GetDefaultSceneRoot) false)
    (Utilities|Casting|CastToArrowComponent _array_element)
    (bind _returnvalue (Game|SpawnActorfromClass "/Game/Blueprints/Enemies/BP_BigEnemy.BP_BigEnemy_C" (Math|Transform|MakeTransform (Transformation|GetWorldLocation _array_element) (Math|Rotator|MakeRotator (.roll (Transformation|GetWorldRotation _array_element)) (.pitch (Transformation|GetWorldRotation _array_element)) (+ (.yaw (Transformation|GetWorldRotation _array_element)) 1.8e+02))) "AlwaysSpawn" 0 0))
    (bind _returnvalue_2 (Actor|GetActorOfClass "/Game/Blueprints/Player/BP_PlayerShip_logic.BP_PlayerShip_logic_C"))
    (Variables|/Game/Blueprints/Objects/BPC_FloatingObject.BPC_FloatingObject_C|SetIs%20Rotated%20By%20Spline (Variables|/Game/Blueprints/Enemies/BP_BigEnemy.BP_BigEnemy_C|GetBPC_FloatingObject _returnvalue) false)
    (Variables|/Game/Blueprints/Objects/BPC_FloatingObject.BPC_FloatingObject_C|SetSpeed%20Forward (Variables|/Game/Blueprints/Enemies/BP_BigEnemy.BP_BigEnemy_C|GetBPC_FloatingObject _returnvalue) (Variables|/Game/Blueprints/Player/BP_PlayerShip_logic.BP_PlayerShip_logic_C|GetStandard%20MSpeed%20Forward _returnvalue_2))))

(event Collision|EventActorBeginOverlap
  (params (OtherActor :type Actor%20Object%20Reference)))

(event EventTick
  (params (DeltaSeconds :type Float%20%28single-precision%29)))

(event EventBeginPlay)

(fn ConstructionScript)