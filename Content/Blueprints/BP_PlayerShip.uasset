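; Player ship pawn that flies forward automatically each tick and steers with the PlayerMoveRight axis.
; Steering banks the ship mesh with a clamped roll Lerp and rolls RotationPoint in world space by the negated input.
; SpeedUp writes a clamped value to HorizontalCurrentSpeed, read only by MovePlayerHorizontal, which nothing here calls, so forward movement uses MovementSpeedForward alone.
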(event EventBeginPlay)

(event Collision|EventActorBeginOverlap
  (params (OtherActor :type Actor%20Object%20Reference)))

(event EventTick
  (params (DeltaSeconds :type Float%20%28single-precision%29))
  (CallFunction|MovePlayerForward))

(event Input|AxisEvents|InputAxisPlayerMoveRight
  (params (AxisValue :type Float%20%28single-precision%29))
  (CallFunction|RotateShip AxisValue)
  (CallFunction|RotateWorld AxisValue))

(event Input|AxisEvents|InputAxisSpeedUp
  (params (AxisValue :type Float%20%28single-precision%29))
  (Variables|Default|SetHorizontal%20Current%20Speed (Math|Float|Clamp(Float) (Math|Float|Lerp AxisValue (* AxisValue (Variables|Default|GetMax%20Forward%20Speed)) (Variables|Default|GetForward%20Velocity)) (Variables|Default|GetMin%20Forward%20Speed) (Variables|Default|GetMax%20Forward%20Speed))))

(fn ConstructionScript)

(fn MovePlayerHorizontal
  (params (Axis%20Value :type Float%20%28double-precision%29))
  (Pawn|Input|AddMovementInput (Transformation|GetActorRightVector) (* Axis%20Value (Variables|Default|GetHorizontal%20Current%20Speed)) true))

(fn RotateShip
  (params (Axis%20Value :type Float%20%28double-precision%29))
  (bind _ship_mesh (Variables|Default|GetShip%20Mesh))
  (bind _target_ship_rotation (Variables|Default|GetTarget%20Ship%20Rotation))
  (bind _relativerotation (Variables|/Script/Engine.SceneComponent|GetRelativeRotation _ship_mesh))
  (Transformation|SetRelativeRotation (Variables|Default|GetShip%20Mesh) (Math|Rotator|MakeRotator (Math|Float|Clamp(Float) (Math|Float|Lerp (.roll _relativerotation) (* Axis%20Value (+ (.roll _relativerotation) (Variables|Default|GetTarget%20Ship%20Rotation))) (Variables|Default|GetShip%20Rotation%20Speed)) (* _target_ship_rotation -1.0) _target_ship_rotation) 0.0 0.0) false false))

(fn RotateWorld
  (params (Axis%20Value :type Float%20%28double-precision%29))
  (Transformation|AddWorldRotation (Variables|Default|GetRotation%20Point) (Math|Rotator|MakeRotator (* (* Axis%20Value (Variables|Default|GetWorld%20Rotation%20Speed)) -1.0) 0.0 0.0) false false))

(fn MovePlayerForward
  (Pawn|Input|AddMovementInput (Transformation|GetActorForwardVector) (Variables|Default|GetMovement%20Speed%20Forward) false))