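; BP_CheckpointTrigger is a checkpoint volume that saves the game when the player ship enters it.
; On Box overlap with BP_PlayerShip_visuals, it creates a new BP_SaveGame and records the score from the ship's LogicReference points.
; It stores the Arrow component's world transform as the player location, rather than the ship's own transform.
; It then writes the save to a fixed slot and prints a confirmation message.
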(event OnComponentBeginOverlap(Box)
  (params (OverlappedComponent :type Primitive%20Component%20Object%20Reference) (OtherActor :type Actor%20Object%20Reference) (OtherComp :type Primitive%20Component%20Object%20Reference) (OtherBodyIndex :type Integer) (bFromSweep :type Boolean) (SweepResult :type Hit%20Result%20Structure%20%28by%20ref%29))
  (bind _asbp_player_ship_visuals (Utilities|Casting|CastToBP_PlayerShip_visuals OtherActor))
  (bind _returnvalue (SaveGame|CreateSaveGameObject "/Game/Blueprints/BP_SaveGame.BP_SaveGame_C"))
  (Variables|Default|SetSave%20Game%20Instance _returnvalue)
  (Variables|/Game/Blueprints/BP_SaveGame.BP_SaveGame_C|SetPlayer%20Score (Variables|Default|GetSave%20Game%20Instance) (Math|Conversions|ToFloat(Integer) (Variables|/Game/Blueprints/Player/BP_PlayerShip_logic.BP_PlayerShip_logic_C|GetPoints (Variables|/Game/Blueprints/Player/BP_PlayerShip_visuals.BP_PlayerShip_visuals_C|GetLogic%20Reference _asbp_player_ship_visuals))))
  (Variables|/Game/Blueprints/BP_SaveGame.BP_SaveGame_C|SetPlayer%20Location (Variables|Default|GetSave%20Game%20Instance) (Transformation|GetWorldTransform (Variables|Default|GetArrow)))
  (SaveGame|SaveGametoSlot (Variables|Default|GetSave%20Game%20Instance) "save1")
  (Development|PrintString "GAME SAVED"))

(fn ConstructionScript)