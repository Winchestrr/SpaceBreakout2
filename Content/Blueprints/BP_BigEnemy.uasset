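; BP_BigEnemy is an enemy actor that explodes and awards points as soon as it receives a DealDamage event, with no health check.
; DealDamage turns off the Box's overlap events, hides the mesh and spawns BP_ExplosionParticle at the root's transform.
; It then adds PointValue to the Points of the BP_PlayerShip_logic found by GetActorOfClass, and destroys itself after a short delay.
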(event EventBeginPlay)

(event Collision|EventActorBeginOverlap
  (params (OtherActor :type Actor%20Object%20Reference)))

(event EventTick
  (params (DeltaSeconds :type Float%20%28single-precision%29)))

(event EventDealDamage
  (params (NewDamage :type Float%20%28double-precision%29))
  (Utilities|FlowControl|Sequence
    (:then_0
      (Variables|/Script/Engine.PrimitiveComponent|SetbGenerateOverlapEvents (Variables|Default|GetBox) false)
      (Rendering|SetVisibility (Variables|Default|GetMesh) false false)
      (Game|SpawnActorfromClass "/Game/Realistic_Starter_VFX_Pack_Vol2/Blueprints/BP_ExplosionParticle.BP_ExplosionParticle_C" (Transformation|GetWorldTransform (Variables|Default|GetDefaultSceneRoot)) "Undefined" 0 0))
    (:then_1
      (bind _returnvalue (Actor|GetActorOfClass "/Game/Blueprints/Player/BP_PlayerShip_logic.BP_PlayerShip_logic_C"))
      (Variables|/Game/Blueprints/Player/BP_PlayerShip_logic.BP_PlayerShip_logic_C|SetPoints _returnvalue (+ (Variables|/Game/Blueprints/Player/BP_PlayerShip_logic.BP_PlayerShip_logic_C|GetPoints _returnvalue) (Variables|Default|GetPoint%20Value))))
    (:then_2
      (Utilities|FlowControl|Delay 3.0)
      (Actor|DestroyActor))))

(fn ConstructionScript)