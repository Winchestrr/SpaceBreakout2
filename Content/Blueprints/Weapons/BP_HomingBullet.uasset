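; Homing bullet actor that flies forward and steers toward an enemy chosen when it spawns.
; On BeginPlay, a multi-sphere trace picks a BP_BigEnemy or BP_SmartEnemy within the Distance threshold.
; The threshold is reassigned to itself, so the last qualifying hit becomes ClosestEnemy, not necessarily the nearest.
; Each Tick moves it without sweep and turns it at constant speed toward that target, with no retargeting or validity check.
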(event Custom|Search%20Enemies
  (bind _defaultsceneroot (Variables|Default|GetDefaultSceneRoot))
  (bind _returnvalue (Transformation|GetWorldLocation _defaultsceneroot))
  (bind _outhits (Collision|MultiSphereTraceByChannel _returnvalue _returnvalue (Variables|Default|GetSearch%20Radius) "TraceTypeQuery1" false 0 "ForOneFrame"))
  (for _array_element _outhits
    (Utilities|Casting|CastToBP_BigEnemy (.HitActor (Collision|BreakHitResult _array_element))
      (:then
        _)
      (:CastFailed
        (Utilities|Casting|CastToBP_SmartEnemy (.HitActor (Collision|BreakHitResult _array_element)))))
    (if (< (Math|Vector|VectorLength (- (Transformation|GetActorLocation (.HitActor (Collision|BreakHitResult _array_element))) (Transformation|GetWorldLocation (Variables|Default|GetDefaultSceneRoot)))) (Variables|Default|GetDistance))
      (Variables|Default|SetDistance (Variables|Default|GetDistance))
      (Variables|Default|SetClosest%20Enemy (.HitActor (Collision|BreakHitResult _array_element))))))

(event EventBeginPlay
  (CallFunction|SearchEnemies))

(event EventTick
  (params (DeltaSeconds :type Float%20%28single-precision%29))
  (Variables|Default|SetDelta%20Seconds DeltaSeconds)
  (Transformation|SetActorLocation (+ (Transformation|GetWorldLocation (Variables|Default|GetDefaultSceneRoot)) (* (Math|Vector|GetForwardVector (Variables|Default|GetDefaultSceneRoot)) (Variables|Default|GetDelta%20Seconds) (Variables|Default|GetBullet%20Speed))) false false)
  (Transformation|SetActorRotation (Class|KismetMathLibrary|RInterptoConstant (Transformation|GetActorRotation) (Math|Conversions|RotationFromXVector (Math|Vector|Normalize (- (Transformation|GetActorLocation (Variables|Default|GetClosest%20Enemy)) (Transformation|GetActorLocation)))) (Variables|Default|GetDelta%20Seconds) (Variables|Default|GetRotation%20Speed))))

(fn ConstructionScript)