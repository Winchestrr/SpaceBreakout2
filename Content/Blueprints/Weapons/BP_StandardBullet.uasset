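; BP_StandardBullet is a projectile actor that deals damage on overlap and expires after a set lifetime.
; It flags its BPCFloatingObject component as a bullet on BeginPlay.
; A Hitbox overlap prints the other actor's name, sends Damage to each of its BPI_Damage components in reverse order, then destroys the bullet.
; A RaycastDown helper only computes trace endpoints along the root's up vector, scaled by RaycastLength.
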(event OnComponentBeginOverlap(Hitbox)
  (params (OverlappedComponent :type Primitive%20Component%20Object%20Reference) (OtherActor :type Actor%20Object%20Reference) (OtherComp :type Primitive%20Component%20Object%20Reference) (OtherBodyIndex :type Integer) (bFromSweep :type Boolean) (SweepResult :type Hit%20Result%20Structure%20%28by%20ref%29))
  (Development|PrintString (Utilities|GetDisplayName OtherActor))
  (bind _arrayelement (Utilities|Array|ReverseforEachLoop (Class|Actor|GetComponentsbyInterface OtherActor "/Game/BPI_Damage.BPI_Damage_C"))
    (:LoopBody
      (Class|BPIDamage|DealDamage(Message) _arrayelement (Variables|Default|GetDamage)))
    (:Completed
      (Actor|DestroyActor))))

(event EventBeginPlay
  (Variables|/Game/Blueprints/Objects/BPC_FloatingObject.BPC_FloatingObject_C|SetIs%20Bullet (Variables|Default|GetBPC_FloatingObject) true)
  (Utilities|FlowControl|Delay (Variables|Default|GetLifetime))
  (Actor|DestroyActor))

(fn ConstructionScript)

(fn RaycastDown
  (bind _defaultsceneroot (Variables|Default|GetDefaultSceneRoot))
  (bind _returnvalue (Transformation|GetWorldLocation _defaultsceneroot))
  (return _returnvalue (+ _returnvalue (* (Math|Vector|GetUpVector (Transformation|GetWorldRotation _defaultsceneroot)) (Variables|Default|GetRaycast%20Length)))))