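; Visual body of the player ship, which trails a separate logic actor each tick using offset, lerped location and rotation.
; Collider overlaps with enemy bullets or big enemies forward damage to the logic actor and play a sound; a separate event plays random left/right damage animations.
; Shoot spawns bullets from muzzle points by bullet count, optionally disabling spline rotation, and Checkpoint notifies the UI with audio.
; Shield overlap is empty; camera-follow and downward-trace code is unwired.
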(event OnComponentBeginOverlap(ShieldCollider)
  (params (OverlappedComponent :type Primitive%20Component%20Object%20Reference) (OtherActor :type Actor%20Object%20Reference) (OtherComp :type Primitive%20Component%20Object%20Reference) (OtherBodyIndex :type Integer) (bFromSweep :type Boolean) (SweepResult :type Hit%20Result%20Structure%20%28by%20ref%29))
  ;[0.3944 1 0.9602] Shield
)

(event OnComponentBeginOverlap(Collider)
  (params (OverlappedComponent :type Primitive%20Component%20Object%20Reference) (OtherActor :type Actor%20Object%20Reference) (OtherComp :type Primitive%20Component%20Object%20Reference) (OtherBodyIndex :type Integer) (bFromSweep :type Boolean) (SweepResult :type Hit%20Result%20Structure%20%28by%20ref%29))
  ;[1 0.1843 0.06453] Get Damage
  (Utilities|Casting|CastToBP_EnemyBullet OtherActor
    (:then
      (Class|BPILogicVisualsConnect|DamagePlayer(Message) (Variables|Default|GetLogic%20Reference) 1.0))
    (:CastFailed
      (Utilities|Casting|CastToBP_SmartEnemyBullet OtherActor
        (:then
          (Class|BPILogicVisualsConnect|DamagePlayer(Message) (Variables|Default|GetLogic%20Reference) 2.0))
        (:CastFailed
          (Utilities|Casting|CastToBP_BigEnemy OtherActor)
          (Class|BPILogicVisualsConnect|DamagePlayer(Message) (Variables|Default|GetLogic%20Reference) 1e+03)))))
  (Class|AkGameplayStatics|PostEvent "/Game/WwiseAudio/Events/Player/P_Damage/Damage_Taken.Damage_Taken" self))

(event Custom|Checkpoint
  (Default|Checkpoint (Variables|Default|GetUI%20Reference))
  ;[0 0.3716 1] SFX_Checkpoint
  (Class|AkGameplayStatics|PostEvent "/Game/WwiseAudio/Events/UI/CheckPoint.CheckPoint" self))

(event Custom|Damage%20Anmiation%20Event
  ;[1 0.5006 0.1517] Get Damage Animations
  (if (Math|Random|RandomBool)
    (Class|ActorSequenceComponent|PlaySequence (Variables|Default|GetGet%20Damage%20Animation%20Right))
    (else
      (Class|ActorSequenceComponent|PlaySequence (Variables|Default|GetGet%20Damage%20Animation%20Left)))))

(event EventBeginPlay
  ;[1 0.326 0.2708] Event Begin
  (Variables|Default|SetNumber%20Of%20Bullets 1))

(event EventShoot
  ;[1 0.2746 0.466] Shooting
  (if (== (Variables|Default|GetNumber%20Of%20Bullets) 1)
    (bind _returnvalue (Game|SpawnActorfromClass "/Game/Blueprints/Weapons/BP_StandardBullet.BP_StandardBullet_C" (Transformation|GetWorldTransform (Variables|Default|GetGunEnd)) "Undefined" 0 0))
    (if (not (Variables|Default|GetAre%20Bullets%20Rotated%20By%20Spline))
      (Variables|/Game/Blueprints/Objects/BPC_FloatingObject.BPC_FloatingObject_C|SetIs%20Rotated%20By%20Spline (Variables|/Game/Blueprints/Weapons/BP_StandardBullet.BP_StandardBullet_C|GetBPC_FloatingObject _returnvalue) false))
    (elif (== (Variables|Default|GetNumber%20Of%20Bullets) 2)
      (bind _returnvalue_2 (Game|SpawnActorfromClass "/Game/Blueprints/Weapons/BP_StandardBullet.BP_StandardBullet_C" (Transformation|GetWorldTransform (Variables|Default|GetGunEnd2)) "Undefined" 0 0))
      (if (Variables|Default|GetAre%20Bullets%20Rotated%20By%20Spline)
        _
        (else
          (Variables|/Game/Blueprints/Objects/BPC_FloatingObject.BPC_FloatingObject_C|SetIs%20Rotated%20By%20Spline (Variables|/Game/Blueprints/Weapons/BP_StandardBullet.BP_StandardBullet_C|GetBPC_FloatingObject _returnvalue_2) false)))
      (bind _returnvalue_3 (Game|SpawnActorfromClass "/Game/Blueprints/Weapons/BP_StandardBullet.BP_StandardBullet_C" (Transformation|GetWorldTransform (Variables|Default|GetGunEnd3)) "Undefined" 0 0))
      (if (not (Variables|Default|GetAre%20Bullets%20Rotated%20By%20Spline))
        (Variables|/Game/Blueprints/Objects/BPC_FloatingObject.BPC_FloatingObject_C|SetIs%20Rotated%20By%20Spline (Variables|/Game/Blueprints/Weapons/BP_StandardBullet.BP_StandardBullet_C|GetBPC_FloatingObject _returnvalue_3) false))
      (elif (>= (Variables|Default|GetNumber%20Of%20Bullets) 3)
        (bind _returnvalue_4 (Game|SpawnActorfromClass "/Game/Blueprints/Weapons/BP_StandardBullet.BP_StandardBullet_C" (Transformation|GetWorldTransform (Variables|Default|GetGunEnd1)) "Undefined" 0 0))
        (if (Variables|Default|GetAre%20Bullets%20Rotated%20By%20Spline)
          _
          (else
            (Variables|/Game/Blueprints/Objects/BPC_FloatingObject.BPC_FloatingObject_C|SetIs%20Rotated%20By%20Spline (Variables|/Game/Blueprints/Weapons/BP_StandardBullet.BP_StandardBullet_C|GetBPC_FloatingObject _returnvalue_4) false)))
        (bind _returnvalue_5 (Game|SpawnActorfromClass "/Game/Blueprints/Weapons/BP_StandardBullet.BP_StandardBullet_C" (Transformation|GetWorldTransform (Variables|Default|GetGunEnd2)) "Undefined" 0 0))
        (if (Variables|Default|GetAre%20Bullets%20Rotated%20By%20Spline)
          _
          (else
            (Variables|/Game/Blueprints/Objects/BPC_FloatingObject.BPC_FloatingObject_C|SetIs%20Rotated%20By%20Spline (Variables|/Game/Blueprints/Weapons/BP_StandardBullet.BP_StandardBullet_C|GetBPC_FloatingObject _returnvalue_5) false)))
        (bind _returnvalue_6 (Game|SpawnActorfromClass "/Game/Blueprints/Weapons/BP_StandardBullet.BP_StandardBullet_C" (Transformation|GetWorldTransform (Variables|Default|GetGunEnd3)) "Undefined" 0 0))
        (if (not (Variables|Default|GetAre%20Bullets%20Rotated%20By%20Spline))
          (Variables|/Game/Blueprints/Objects/BPC_FloatingObject.BPC_FloatingObject_C|SetIs%20Rotated%20By%20Spline (Variables|/Game/Blueprints/Weapons/BP_StandardBullet.BP_StandardBullet_C|GetBPC_FloatingObject _returnvalue_6) false))))))

(event EventTick
  (params (DeltaSeconds :type Float%20%28single-precision%29))
  (bind (_player_location _player_rotation) (CallFunction|GetDesiredMeshLocation))
  (Transformation|SetWorldRotation (Variables|Default|GetRoot) _player_rotation false false)
  (Transformation|SetWorldLocation (Variables|Default|GetRoot) _player_location false false))

(fn ConstructionScript)

(fn GetDesiredMeshLocation
  (bind _logic_reference (Variables|Default|GetLogic%20Reference))
  (bind _returnvalue (Transformation|GetActorLocation _logic_reference))
  (return (Math|Vector|Lerp(Vector) (Transformation|GetActorLocation) (Math|Vector|MakeVector (+ (.x _returnvalue) (Variables|Default|GetMesh%20X%20Offset)) (.y _returnvalue) (+ (Variables|Default|GetMesh%20Z%20Offset) (.z _returnvalue))) (Variables|Default|GetMesh%20Location%20Lerp%20Speed)) (Math|Rotator|Lerp(Rotator) (Transformation|GetActorRotation) (Transformation|GetActorRotation _logic_reference) (Variables|Default|GetMesh%20Rotation%20Lerp%20Speed))))

(fn GetDesiredCameraLocation
  (bind _logic_reference (Variables|Default|GetLogic%20Reference))
  (bind _returnvalue (Transformation|GetActorLocation _logic_reference))
  (return (Math|Vector|MakeVector (+ (.x _returnvalue) (Variables|Default|GetCamera%20X%20Offset)) (.y _returnvalue) (.z _returnvalue)) (Transformation|GetActorRotation _logic_reference)))

(fn RaycastDown
  (bind _root (Variables|Default|GetRoot))
  (bind _returnvalue (Transformation|GetWorldLocation _root))
  (return _returnvalue (+ _returnvalue (* (Math|Vector|GetUpVector (Transformation|GetWorldRotation _root)) -3e+03))))