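; Player ship logic for a track-hovering shooter: handles steering, speed, gravity inversion, firing, health and energy, with Wwise engine audio.
; Spawns a separate visuals actor for mesh banking and shooting.
; Each tick moves the ship, traces along its gravity axis to hold height and align to the surface, optionally taking yaw from BP_Spline.
; Losing the track or dying from damage or energy drain triggers falling, slow-motion camera and game over.
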(event Custom|Change%20Camera%20To%20Battle)

(event Custom|Start%20Energy%20Counter
  ;[0.6315 1 0.1435] Energy
  (Variables|Energy|SetCurrent%20Energy (Variables|Energy|GetMax%20Energy))
  (Utilities|FlowControl|DoOnce false
    (:Completed
      (if (or (Variables|Input|GetIs%20Speeding%20Down) (Variables|Input|GetIs%20Speeding%20Up)) :!label _label
        (Utilities|FlowControl|Delay (Variables|Energy|GetFast%20Energy%20Drain%20Delay))
        (else
          (Utilities|FlowControl|Delay (Variables|Energy|GetStandard%20Energy%20Drain%20Delay))))
      (Math|Float|DecrementFloat (Variables|Energy|GetCurrent%20Energy)
        (:%20%20
          (Development|PrintString (Utilities|String|Append "Current energy: " (Utilities|String|ToString(Float) (Variables|Energy|GetCurrent%20Energy))) true true "(R=0.000000,G=0.660000,B=1.000000,A=1.000000)" 2.0 "Energy")
          (if (<= (Variables|Energy|GetCurrent%20Energy) 0.0)
            (Variables|Default|SetIs%20Dead true)
            (else
              (goto _label))))))))

(event EventBeginPlay
  ;[1 0.4007 0.2807] Event Begin
  (bind _returnvalue (Game|SpawnActorfromClass "/Game/Blueprints/Player/BP_PlayerShip_visuals.BP_PlayerShip_visuals_C" (Transformation|GetWorldTransform (Variables|Default|GetRoot)) "Undefined" 0 0))
  (bind _output_get (Variables|References|SetVisuals%20Reference _returnvalue))
  (Variables|/Game/Blueprints/Player/BP_PlayerShip_visuals.BP_PlayerShip_visuals_C|SetLogic%20Reference _output_get self)
  (Variables|References|SetGun%20Reference (Variables|/Game/Blueprints/Player/BP_PlayerShip_visuals.BP_PlayerShip_visuals_C|GetGun%20Reference (Variables|References|GetVisuals%20Reference)))
  (CallFunction|StartEnergyCounter)
  (bind _returnvalue_2 (Actor|GetActorOfClass "/Game/Blueprints/BP_Spline.BP_Spline_C"))
  (bind _output_get_2 (Variables|Default|SetMovement%20Spline _returnvalue_2))
  (Class|BPISpawnerPlayerConnect|TransferLogicReference(Message) _output_get_2 self)
  ;;[0 0.5532 1] SFX_EngineStart
  (Class|AkGameplayStatics|PostEvent "/Game/WwiseAudio/Events/EngineStart.EngineStart" self))

(event EventDamagePlayer
  (params (Damage%20Amount :type Float%20%28double-precision%29))
  ;[0.3441 1 0.3734] Get Inputs
  (CallFunction|DealPlayerDamage 1e+01))

(event EventTick
  (params (DeltaSeconds :type Float%20%28single-precision%29))
  (bind (_startposition _endposition) (CallFunction|RaycastDown))
  (bind _springarm (Variables|Default|GetSpringArm))
  (bind _root (Variables|Default|GetRoot))
  (bind _relativerotation (Variables|/Script/Engine.SceneComponent|GetRelativeRotation _springarm))
  ;[0.314 0.1352 0.08156] Event Tick
  (Variables|Default|SetDelta%20Seconds DeltaSeconds)
  (Utilities|FlowControl|Sequence
    (:then_0
      ;[0.3702 1 0.6408] Setting Speed and Camera
      (if (Variables|Input|GetIs%20Speeding%20Up)
        (Variables|Forward|SetCurrent%20MSpeed%20Forward (Math|Float|Lerp (Variables|Forward|GetCurrent%20MSpeed%20Forward) (Variables|Forward|GetMax%20MSpeed%20Forward) (Variables|Forward|GetAcceleration%20Rate)))
        (elif (Variables|Input|GetIs%20Speeding%20Down)
          (Variables|Forward|SetCurrent%20MSpeed%20Forward (Math|Float|Lerp (Variables|Forward|GetCurrent%20MSpeed%20Forward) (Variables|Forward|GetMin%20MSpeed%20Forward) (Variables|Forward|GetAcceleration%20Rate)))
          (else
            (Variables|Forward|SetCurrent%20MSpeed%20Forward (Math|Float|Lerp (Variables|Forward|GetCurrent%20MSpeed%20Forward) (Variables|Forward|GetStandard%20MSpeed%20Forward) (Variables|Forward|GetAcceleration%20Rate))))))
      ;;[0 0.466 1] SFX_Speed
      (Class|AkGameplayStatics|SetRTPCValue "/Game/WwiseAudio/RTPC/Speed.Speed" (Variables|Forward|GetCurrent%20MSpeed%20Forward) 0 self))
    (:then_1
      ;[0.1887 0.7885 1] Movement
      (if (Variables|Default|GetCan%20Move)
        (if (Variables|Default|GetPlayerInputEnabled)
          (CallFunction|SetLocationbyInput (Variables|Default|GetDelta%20Seconds))
          (bind (_outhit _returnvalue) (Collision|LineTraceByChannel _startposition _endposition "TraceTypeQuery3" true 0 "None"))
          (if _returnvalue
            (if (Variables|Default|GetIs%20Dead)
              (Variables|Default|SetPlayerInputEnabled false :!label _label)
              ;;[1 0.2392 0.1395] Game Over Animation
              (Utilities|Time|SetGlobalTimeDilation (Math|Float|Lerp (Class|GameplayStatics|GetGlobalTimeDilation) 0.0 0.05) :!label _label_2)
              (Variables|/Script/Engine.SpringArmComponent|SetTargetArmLength _springarm (Math|Float|Lerp (Variables|/Script/Engine.SpringArmComponent|GetTargetArmLength _springarm) 5e+02 0.1))
              (Transformation|SetRelativeRotation _springarm (Math|Rotator|MakeRotator 0.0 (Math|Float|Lerp (.pitch _relativerotation) -9e+01 0.5) (Math|Float|Lerp (.yaw _relativerotation) 3e+01 0.5)) false false)
              (Utilities|FlowControl|DoOnce false
                (:Completed
                  (Default|CallGameOver)
                  (Variables|/Script/Engine.PlayerController|SetbShowMouseCursor (Game|GetPlayerController 0) true)
                  ;;;[0 0.3971 1] SFX_Stop
                  (Class|AkGameplayStatics|PostEvent "/Game/WwiseAudio/Events/EngineStop.EngineStop" self)))
              (else
                (if (Variables|Default|GetIs%20Turning%20By%20Spline)
                  (LogicMovement|RotateLogicbyRaycast (.ImpactNormal (Collision|BreakHitResult _outhit)) (Variables|Default|GetDelta%20Seconds)))
                (LogicMovement|SetLogicHeight (.ImpactPoint (Collision|BreakHitResult _outhit)) (.ImpactNormal (Collision|BreakHitResult _outhit)))
                (CallFunction|RotateShip (Variables|Horizontal|GetMove%20Right%20Axis))
                (if (== (Math|Float|Sign(Float) (Variables|Default|GetInverted%20Gravity%20Vector)) -1.0)
                  (Math|Float|NegateFloat (Variables|Default|GetInverted%20Gravity%20Vector)))))
            (else
              (goto _label)))
          (else
            ;;[0.9614 1 0.6362] Fall
            (Transformation|SetWorldLocation (Variables|Default|GetRoot) (+ (Transformation|GetWorldLocation _root) (* (Math|Vector|GetUpVector _root) -1.0 (Variables|Default|GetFallSpeed) (Variables|Default|GetDelta%20Seconds)) (* (Math|Vector|GetForwardVector _root) (Variables|Default|GetFallSpeedForward) (Variables|Default|GetDelta%20Seconds))) false false)
            (goto _label_2)))))
    (:then_2
      ;[1 0.9361 0.3207] Shooting
      (if (Variables|Input|GetIs%20Shooting)
        (if (Variables|Default|GetCan%20Shoot)
          (Utilities|FlowControl|Sequence
            (:then_0
              (Variables|Default|SetCan%20Shoot false)
              (Class|BPIShooting|Shoot(Message) (Variables|References|GetVisuals%20Reference)))
            (:then_1
              (Utilities|FlowControl|Delay (Variables|Default|GetTime%20Between%20Shots))
              (Variables|Default|SetCan%20Shoot true))))))
    (:then_3)))

(event Input|ActionEvents|InputActionShoot
  (params (Key :type Key%20Structure :default "None"))
  ;[0.3441 1 0.3734] Get Inputs
  (:Pressed
    (Variables|Input|SetIs%20Shooting true))
  (:Released
    (Variables|Input|SetIs%20Shooting false)))

(event Input|ActionEvents|InputActionSpeedUpKey
  (params (Key :type Key%20Structure :default "None"))
  ;[0.3441 1 0.3734] Get Inputs
  (:Pressed
    (if (not (Variables|Input|GetIs%20Speeding%20Down))
      (Variables|Input|SetIs%20Speeding%20Up true)))
  (:Released
    (Variables|Input|SetIs%20Speeding%20Up false)))

(event Input|ActionEvents|InputActionSpeedDownKey
  (params (Key :type Key%20Structure :default "None"))
  ;[0.3441 1 0.3734] Get Inputs
  (:Pressed
    (if (not (Variables|Input|GetIs%20Speeding%20Up))
      (Variables|Input|SetIs%20Speeding%20Down true)))
  (:Released
    (Variables|Input|SetIs%20Speeding%20Down false)))

(event Input|ActionEvents|InputActionInvertGravity
  (params (Key :type Key%20Structure :default "None"))
  ;[0.3441 1 0.3734] Get Inputs
  (:Pressed
    (Variables|Input|SetIs%20Gravity%20Inverted (not (Variables|Input|GetIs%20Gravity%20Inverted)))
    (Math|Float|NegateFloat (Variables|Default|GetInverted%20Gravity%20Vector))))

(event Input|ActionEvents|InputActionDebugDealDamage
  (params (Key :type Key%20Structure :default "None"))
  ;[0.3441 1 0.3734] Get Inputs
)

(event Input|AxisEvents|InputAxisSpeedUp
  (params (AxisValue :type Float%20%28single-precision%29))
  ;[0.3441 1 0.3734] Get Inputs
  (Variables|Forward|SetSpeed%20Up%20Axis AxisValue))

(event Input|AxisEvents|InputAxisPlayerRotateRight
  (params (AxisValue :type Float%20%28single-precision%29))
  ;[0.3441 1 0.3734] Get Inputs
  (Variables|Horizontal|SetMove%20Right%20Axis AxisValue))

(event Input|KeyboardEvents|C
  (params (Key :type Key%20Structure :default "None"))
  (:Pressed
    (if (Variables|Default|GetIs%20Battle%20Camera%20Active)
      (Variables|Default|SetIs%20Battle%20Camera%20Active false)
      (Development|PrintString "battle camera disabled")
      (else
        (Variables|Default|SetIs%20Battle%20Camera%20Active true)
        (Development|PrintString "battle camera enabled")))))

(fn ConstructionScript)

(fn MoveLogicHorizontal
  (params (Axis%20Value :type Float%20%28double-precision%29))
  (Pawn|Input|AddMovementInput (+ (* (Transformation|GetActorRightVector) (Variables|Horizontal|GetMove%20Right%20Axis)) (* (Transformation|GetActorForwardVector) (Variables|Forward|GetSpeed%20Up%20Axis))) Axis%20Value false))

(fn RotateShip
  (params (Axis%20Value :type Float%20%28double-precision%29))
  (bind _visuals_reference (Variables|References|GetVisuals%20Reference))
  (bind _target_ship_rotation (Variables|Rotation|GetTarget%20Ship%20Rotation))
  (bind _target_ship_rotation_2 (Variables|Rotation|GetTarget%20Ship%20Rotation))
  (bind _ship_rotation_speed (Variables|Rotation|GetShip%20Rotation%20Speed))
  (bind _returnvalue (* _target_ship_rotation_2 -1.0))
  (bind _returnvalue_2 (* _target_ship_rotation Axis%20Value))
  (bind _mesh (Variables|/Game/Blueprints/Player/BP_PlayerShip_visuals.BP_PlayerShip_visuals_C|GetMesh _visuals_reference))
  (bind _returnvalue_3 (Transformation|GetRelativeTransform _mesh))
  (bind _returnvalue_4 (Math|Float|Lerp (.pitch (.rotation _returnvalue_3)) _returnvalue_2 _ship_rotation_speed))
  (bind _returnvalue_5 (Math|Float|Clamp(Float) _returnvalue_4 _returnvalue _target_ship_rotation_2))
  (Transformation|SetRelativeRotation _mesh (Math|Rotator|MakeRotator (.roll (.rotation _returnvalue_3)) _returnvalue_5 (.yaw (.rotation _returnvalue_3))) false false)
  (Class|AkGameplayStatics|SetRTPCValue "/Game/WwiseAudio/RTPC/Glide.Glide" (Math|Float|Absolute(Float) _returnvalue_5) 0 self))

(fn MoveLogicForward
  (Pawn|Input|AddMovementInput (Transformation|GetActorForwardVector) 1.0 true))

(fn RotateLogicbyRaycast
  (params (Normal :type Vector%20%28by%20ref%29) (DeltaTime :type Float%20%28single-precision%29))
  (bind _movement_spline (Variables|Default|GetMovement%20Spline))
  (bind _root (Variables|Default|GetRoot))
  (bind _returnvalue (Transformation|GetWorldLocation _root))
  (bind _spline (Variables|/Game/Blueprints/BP_Spline.BP_Spline_C|GetSpline _movement_spline))
  (bind _returnvalue_2 (Class|SplineComponent|FindInputKeyClosesttoWorldLocation _spline _returnvalue))
  (Variables|Default|SetClosest%20Input%20Key _returnvalue_2)
  (Transformation|SetWorldRotation _root (Math|Interpolation|RInterpTo (Transformation|GetWorldRotation _root) (Math|Rotator|MakeRotator (.Roll (Math|Rotator|BreakRotator (Math|Rotator|MakeRotfromXZ (Math|Vector|GetForwardVector _root) Normal))) (.Pitch (Math|Rotator|BreakRotator (Class|KismetMathLibrary|MakeRotfromYZ (Math|Vector|GetRightVector _root) Normal))) (.yaw (Class|SplineComponent|GetRotationatSplineInputKey _spline _returnvalue_2 "World"))) DeltaTime 0.0) false false))

(fn RaycastDown
  (bind _root (Variables|Default|GetRoot))
  (bind _returnvalue (Transformation|GetWorldLocation _root))
  (return _returnvalue (+ _returnvalue (* (Math|Vector|GetUpVector (Transformation|GetWorldRotation _root)) (Variables|Default|GetRaycast%20Length) (Variables|Default|GetInverted%20Gravity%20Vector)))))

(fn SetLogicHeight
  (params (Impact%20Point :type Vector) (Impact%20Normal :type Vector))
  (Transformation|SetWorldLocation (Variables|Default|GetRoot) (+ Impact%20Point (* (Math|Vector|Normalize Impact%20Normal) 2e+02)) false false))

(fn SetLocationbyInput
  (params (Delta%20Time :type Float%20%28single-precision%29))
  (Transformation|SetActorLocation (+ (Transformation|GetActorLocation) (* (Transformation|GetActorRightVector) (Variables|Horizontal|GetMove%20Right%20Axis) (Variables|Horizontal|GetMovement%20Speed%20Horizontal) Delta%20Time) (* (Transformation|GetActorForwardVector) (Variables|Forward|GetCurrent%20MSpeed%20Forward) Delta%20Time)) false false)
  (return))

(fn SetTimeBetweenShots
  (params (NewValue :type Float%20%28double-precision%29))
  (Variables|Default|SetTime%20Between%20Shots NewValue))

(fn DealPlayerDamage
  (params (Damage :type Float%20%28double-precision%29))
  (bind _player_health (Variables|PlayerStats|GetPlayer%20Health))
  (Math|Float|DecrementFloat _player_health
    (:%20%20
      (if (<= _player_health 0.0)
        (Variables|Default|SetIs%20Dead true)
        (else
          (Variables|Default|SetIs%20Dead false)))
      (return (Variables|Default|GetIs%20Dead)))))