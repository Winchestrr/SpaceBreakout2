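; BP_BlueExplosionParticle is an effect actor that plays a Niagara effect, by its name a blue explosion.
; On BeginPlay it activates the Niagara component, waits a fixed delay and deactivates it, without destroying the actor.
; A disconnected chain that would replay a VFX component at an interval or destroy the actor, depending on IsLoop, never runs.
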(event EventBeginPlay
  (bind _niagara (Variables|Default|GetNiagara))
  (Components|Activation|Activate _niagara false)
  (Utilities|FlowControl|Delay 1e+01)
  (Components|Activation|Deactivate _niagara))

(event Collision|EventActorBeginOverlap
  (params (OtherActor :type Actor%20Object%20Reference)))

(event EventTick
  (params (DeltaSeconds :type Float%20%28single-precision%29)))

(fn ConstructionScript)