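; BP_EnemySplineActivator is a trigger volume that launches enemy spline entrances when the player ship reaches it.
; A box overlap filters for BP_PlayerShip_visuals and passes through a DoOnce, so activation fires a single time.
; It then calls StartEntering on every entry in the big enemy spline list, followed by every entry in the smart enemy spline list.
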(event OnComponentBeginOverlap(Box)
  (params (OverlappedComponent :type Primitive%20Component%20Object%20Reference) (OtherActor :type Actor%20Object%20Reference) (OtherComp :type Primitive%20Component%20Object%20Reference) (OtherBodyIndex :type Integer) (bFromSweep :type Boolean) (SweepResult :type Hit%20Result%20Structure%20%28by%20ref%29))
  (bind _big_enemy_spline_list (Variables|Default|GetBig%20Enemy%20Spline%20List))
  (bind _smart_enemy_spline_list (Variables|Default|GetSmart%20Enemy%20Spline%20List))
  (Utilities|Casting|CastToBP_PlayerShip_visuals OtherActor)
  (Utilities|FlowControl|DoOnce false
    (:Completed
      (Utilities|FlowControl|Sequence
        (:then_0
          (for (_ _array_index) _big_enemy_spline_list
            (Default|StartEntering (Utilities|Array|Get(acopy) _big_enemy_spline_list _array_index))))
        (:then_1
          (for (_ _array_index_2) _smart_enemy_spline_list
            (Default|StartEntering (Utilities|Array|Get(acopy) _smart_enemy_spline_list _array_index_2))))))))

(fn ConstructionScript)