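; BP_BattleArenaTrigger is a trigger volume that switches the player ship from spline travel into battle arena mode.
; When a Player-tagged BP_PlayerShip_visuals overlaps its collider, it turns off spline-based turning and bullet rotation and stops BP_Spline spawning enemies.
; It then snaps the ship logic's yaw to the trigger's yaw minus 90 degrees and switches to the battle camera.
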(event OnComponentBeginOverlap(Collider)
  (params (OverlappedComponent :type Primitive%20Component%20Object%20Reference) (OtherActor :type Actor%20Object%20Reference) (OtherComp :type Primitive%20Component%20Object%20Reference) (OtherBodyIndex :type Integer) (bFromSweep :type Boolean) (SweepResult :type Hit%20Result%20Structure%20%28by%20ref%29))
  (if (Actor|ActorHasTag OtherActor "Player")
    (Utilities|FlowControl|Sequence
      (:then_0
        (bind _asbp_player_ship_visuals (Utilities|Casting|CastToBP_PlayerShip_visuals OtherActor))
        (Variables|/Game/Blueprints/Player/BP_PlayerShip_logic.BP_PlayerShip_logic_C|SetIs%20Turning%20By%20Spline (Variables|/Game/Blueprints/Player/BP_PlayerShip_visuals.BP_PlayerShip_visuals_C|GetLogic%20Reference _asbp_player_ship_visuals) false)
        (bind _returnvalue (Actor|GetActorOfClass "/Game/Blueprints/Player/BP_PlayerShip_visuals.BP_PlayerShip_visuals_C"))
        (Variables|/Game/Blueprints/Player/BP_PlayerShip_visuals.BP_PlayerShip_visuals_C|SetAre%20Bullets%20Rotated%20By%20Spline _returnvalue false)
        (bind _returnvalue_2 (Actor|GetActorOfClass "/Game/Blueprints/BP_Spline.BP_Spline_C"))
        (Variables|/Game/Blueprints/BP_Spline.BP_Spline_C|SetCan%20Enemies%20Be%20Spawned _returnvalue_2 false)
        (Transformation|SetWorldRotation (Variables|/Game/Blueprints/Player/BP_PlayerShip_logic.BP_PlayerShip_logic_C|GetRoot (Variables|/Game/Blueprints/Player/BP_PlayerShip_visuals.BP_PlayerShip_visuals_C|GetLogic%20Reference _asbp_player_ship_visuals)) (Math|Rotator|MakeRotator (.roll (Transformation|GetWorldRotation (Variables|/Game/Blueprints/Player/BP_PlayerShip_logic.BP_PlayerShip_logic_C|GetRoot (Variables|/Game/Blueprints/Player/BP_PlayerShip_visuals.BP_PlayerShip_visuals_C|GetLogic%20Reference _asbp_player_ship_visuals)))) (.pitch (Transformation|GetWorldRotation (Variables|/Game/Blueprints/Player/BP_PlayerShip_logic.BP_PlayerShip_logic_C|GetRoot (Variables|/Game/Blueprints/Player/BP_PlayerShip_visuals.BP_PlayerShip_visuals_C|GetLogic%20Reference _asbp_player_ship_visuals)))) (- (.yaw (Transformation|GetWorldRotation (Variables|Default|GetDefaultSceneRoot))) 9e+01)) false false))
      (:then_1
        (Default|ChangeCameratoBattle (Variables|/Game/Blueprints/Player/BP_PlayerShip_visuals.BP_PlayerShip_visuals_C|GetLogic%20Reference _asbp_player_ship_visuals))))))

(event EventBeginPlay)

(event Collision|EventActorBeginOverlap
  (params (OtherActor :type Actor%20Object%20Reference)))

(event EventTick
  (params (DeltaSeconds :type Float%20%28single-precision%29)))

(fn ConstructionScript)