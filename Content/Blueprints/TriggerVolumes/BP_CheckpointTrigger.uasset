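; Checkpoint trigger volume that saves the player ship's progress when the ship overlaps its box.
; On overlap it loads the "save1" slot, or creates a new BP_SaveGame if none exists.
; It writes its checkpoint number, current goal, points and timer, saves, hides its mesh and calls the ship's Checkpoint event.
; An older save path that stored the arrow's transform is left disconnected.
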(event OnComponentBeginOverlap(Box)
  (params (OverlappedComponent :type Primitive%20Component%20Object%20Reference) (OtherActor :type Actor%20Object%20Reference) (OtherComp :type Primitive%20Component%20Object%20Reference) (OtherBodyIndex :type Integer) (bFromSweep :type Boolean) (SweepResult :type Hit%20Result%20Structure%20%28by%20ref%29))
  (bind _asbp_player_ship_visuals (Utilities|Casting|CastToBP_PlayerShip_visuals OtherActor))
  (Variables|Default|SetVisuals%20Reference _asbp_player_ship_visuals)
  (bind _returnvalue (SaveGame|DoesSaveGameExist "save1"))
  (if _returnvalue
    ;[0.3185 1 0.2299] Save Exists
    (bind _returnvalue_2 (SaveGame|LoadGamefromSlot "save1"))
    (bind _asbp_save_game (Utilities|Casting|CastToBP_SaveGame _returnvalue_2))
    (Variables|Default|SetSave%20Game%20Reference _asbp_save_game)
    (else
      ;[1 0.1335 0.1036] Save Does Not Exists
      (bind _returnvalue_3 (SaveGame|CreateSaveGameObject "/Game/Blueprints/BP_SaveGame.BP_SaveGame_C"))
      (Variables|Default|SetSave%20Game%20Reference _returnvalue_3)))
  ;[0.2764 0.9202 1] Save Game
  (Variables|/Game/Blueprints/BP_SaveGame.BP_SaveGame_C|SetCurrent%20Player%20Start (Variables|Default|GetSave%20Game%20Reference) (Variables|Default|GetCheckpoint%20Number))
  (Variables|/Game/Blueprints/BP_SaveGame.BP_SaveGame_C|SetCurrent%20Goal (Variables|Default|GetSave%20Game%20Reference) (Variables|/Game/Blueprints/Player/BP_PlayerShip_visuals.BP_PlayerShip_visuals_C|GetCurrent%20Goal%20Text (Variables|Default|GetVisuals%20Reference)))
  (Variables|/Game/Blueprints/BP_SaveGame.BP_SaveGame_C|SetPlayer%20Score (Variables|Default|GetSave%20Game%20Reference) (Math|Conversions|ToFloat(Integer) (Variables|/Game/Blueprints/Player/BP_PlayerShip_logic.BP_PlayerShip_logic_C|GetPoints (Variables|/Game/Blueprints/Player/BP_PlayerShip_visuals.BP_PlayerShip_visuals_C|GetLogic%20Reference (Variables|Default|GetVisuals%20Reference)))))
  (Variables|/Game/Blueprints/BP_SaveGame.BP_SaveGame_C|SetTimer (Variables|Default|GetSave%20Game%20Reference) (Variables|/Game/Blueprints/Player/BP_PlayerShip_logic.BP_PlayerShip_logic_C|GetTimeText (Variables|/Game/Blueprints/Player/BP_PlayerShip_visuals.BP_PlayerShip_visuals_C|GetLogic%20Reference (Variables|Default|GetVisuals%20Reference))))
  (SaveGame|SaveGametoSlot (Variables|Default|GetSave%20Game%20Reference) "save1")
  (Rendering|SetVisibility (Variables|Default|GetMesh) false false)
  (Default|Checkpoint (Variables|Default|GetVisuals%20Reference)))

(fn ConstructionScript)