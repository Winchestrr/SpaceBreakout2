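; BP_ChangeSideTrigger is a trigger volume that flips the roll of any actor entering its box.
; On overlap, an exact zero-roll check selects the "Rotate right" or "Rotate left" timeline, with a debug print.
; The chosen timeline drives the actor's rotation through its roll value each update.
; A CanBeRotated flag blocks retriggering until that timeline finishes.
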(event OnComponentBeginOverlap(Box)
  (params (OverlappedComponent :type Primitive%20Component%20Object%20Reference) (OtherActor :type Actor%20Object%20Reference) (OtherComp :type Primitive%20Component%20Object%20Reference) (OtherBodyIndex :type Integer) (bFromSweep :type Boolean) (SweepResult :type Hit%20Result%20Structure%20%28by%20ref%29))
  (if (Variables|Default|GetCan%20Be%20Rotated)
    (if (== (.roll (Transformation|GetActorRotation OtherActor)) 0.0)
      (Variables|Default|SetCan%20Be%20Rotated false)
      (Development|PrintString "Rotate right")
      (bind _rotation (Timeline|Rotation%20Right%20Timeline PlayFromStart)
        (:Update
          (Transformation|SetActorRotation OtherActor (Math|Rotator|MakeRotator _rotation 0.0 0.0)))
        (:Finished
          (Variables|Default|SetCan%20Be%20Rotated true :!label _label)))
      (else
        (Variables|Default|SetCan%20Be%20Rotated false)
        (Development|PrintString "Rotate left")
        (bind _rotation_2 (Timeline|Timeline_0 PlayFromStart)
          (:Update
            (Transformation|SetActorRotation OtherActor (Math|Rotator|MakeRotator _rotation_2 0.0 0.0)))
          (:Finished
            (goto _label)))))))

(event EventBeginPlay)

(event Collision|EventActorBeginOverlap
  (params (OtherActor :type Actor%20Object%20Reference)))

(event EventTick
  (params (DeltaSeconds :type Float%20%28single-precision%29)))

(fn ConstructionScript)