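; Damage-up power-up Blueprint that temporarily boosts the collecting character's damage.
; On activation it runs the parent logic, caches the current Damage on the base logic reference, multiplies it by the power-up value and posts a Wwise pickup sound.
; When the power-up ends it restores the cached damage; UI icon reset calls exist in both graphs but are disconnected.
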(fn ConstructionScript)

(fn CustomPowerUpLogic
  (bind _self self)
  (bind _base_logic_reference (Variables|Default|GetBase%20Logic%20Reference))
  (|CallParentFunction)
  (bind _output_get (Variables|Default|SetOld%20Damage%20Value (Variables|/Game/Blueprints/Player/BP_PlayerShip_logic.BP_PlayerShip_logic_C|GetDamage _base_logic_reference)))
  (Variables|/Game/Blueprints/Player/BP_PlayerShip_logic.BP_PlayerShip_logic_C|SetDamage _base_logic_reference (* _output_get (Variables|Default|GetPower%20Up%20Value)))
  ;[0 0.4233 1] SFX_PickUP
  (Class|AkGameplayStatics|SetOcclusionRefreshInterval 0.0 _self)
  (Class|AkGameplayStatics|PostEvent "/Game/WwiseAudio/Events/Power_Ups/PickUp_PowerUp.PickUp_PowerUp" _self)
  (return))

(fn PowerUpEndLogic
  (|CallParentFunction)
  (Variables|/Game/Blueprints/Player/BP_PlayerShip_logic.BP_PlayerShip_logic_C|SetDamage (Variables|Default|GetBase%20Logic%20Reference) (Variables|Default|GetOld%20Damage%20Value))
  (return))