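; BP_PU_AddHP is a power-up that adds health to the player on pickup.
; Its CustomPowerUpLogic override calls the parent, then adds AddHPAmount to PlayerHealth through BaseLogicReference.
; It compares the result to MaxPlayerHealth, but both branches add the full amount, so health is not capped here.
; It then disables Wwise occlusion refresh on itself and posts the pickup sound event.
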(fn ConstructionScript)

(fn CustomPowerUpLogic
  (bind _self self)
  (|CallParentFunction)
  (if (<= (+ (Variables|/Game/Blueprints/Player/BP_PlayerShip_logic.BP_PlayerShip_logic_C|GetPlayer%20Health (Variables|Default|GetBase%20Logic%20Reference)) (Variables|Default|GetAdd%20HP%20Amount)) (Variables|/Game/Blueprints/Player/BP_PlayerShip_logic.BP_PlayerShip_logic_C|GetMax%20Player%20Health (Variables|Default|GetBase%20Logic%20Reference)))
    (Variables|/Game/Blueprints/Player/BP_PlayerShip_logic.BP_PlayerShip_logic_C|SetPlayer%20Health (Variables|Default|GetBase%20Logic%20Reference) (+ (Variables|/Game/Blueprints/Player/BP_PlayerShip_logic.BP_PlayerShip_logic_C|GetPlayer%20Health (Variables|Default|GetBase%20Logic%20Reference)) (Variables|Default|GetAdd%20HP%20Amount)))
    (else
      (Variables|/Game/Blueprints/Player/BP_PlayerShip_logic.BP_PlayerShip_logic_C|SetPlayer%20Health (Variables|Default|GetBase%20Logic%20Reference) (+ (Variables|/Game/Blueprints/Player/BP_PlayerShip_logic.BP_PlayerShip_logic_C|GetPlayer%20Health (Variables|Default|GetBase%20Logic%20Reference)) (Variables|Default|GetAdd%20HP%20Amount)))))
  ;[0 0.4233 1] SFX_PickUP
  (Class|AkGameplayStatics|SetOcclusionRefreshInterval 0.0 _self)
  (Class|AkGameplayStatics|PostEvent "/Game/WwiseAudio/Events/Power_Ups/PickUp_PowerUp.PickUp_PowerUp" _self)
  (return))