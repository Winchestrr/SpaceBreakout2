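; Power-up Blueprint that temporarily changes the fire rate by scaling TimeBetweenShots on the referenced base logic.
; On activation it caches the current time between shots, multiplies it by the power-up value, and posts the Wwise pickup sound with occlusion refresh set to zero.
; When the power-up ends it writes the cached value back, with both steps extending the parent power-up logic.
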(fn ConstructionScript)

(fn CustomPowerUpLogic
  (bind _self self)
  (|CallParentFunction)
  (Variables|Default|SetOld%20TBS%20Value (Variables|/Game/Blueprints/Player/BP_PlayerShip_logic.BP_PlayerShip_logic_C|GetTime%20Between%20Shots (Variables|Default|GetBase%20Logic%20Reference)))
  (Default|SetTimeBetweenShots (Variables|Default|GetBase%20Logic%20Reference) (* (Variables|Default|GetOld%20TBS%20Value) (Variables|Default|GetPower%20Up%20Value)))
  ;[0 0.4233 1] SFX_PickUP
  (Class|AkGameplayStatics|SetOcclusionRefreshInterval 0.0 _self)
  (Class|AkGameplayStatics|PostEvent "/Game/WwiseAudio/Events/Power_Ups/PickUp_PowerUp.PickUp_PowerUp" _self)
  (return))

(fn PowerUpEndLogic
  (|CallParentFunction)
  (Default|SetTimeBetweenShots (Variables|Default|GetBase%20Logic%20Reference) (Variables|Default|GetOld%20TBS%20Value))
  (return))