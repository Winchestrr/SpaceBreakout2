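; Base power-up pickup that plays a float animation and reacts when the player ship's visuals actor overlaps its collider.
; On pickup it caches the ship's visual and logic references, runs the empty CustomPowerUpLogic hook meant for children, and spawns a particle.
; Timed power-ups then hide the mesh, disable overlaps, wait for the duration and call the empty PowerUpEndLogic hook.
; The actor destroys itself afterward, or immediately when it has no duration.
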(event OnComponentBeginOverlap(Collider)
  (params (OverlappedComponent :type Primitive%20Component%20Object%20Reference) (OtherActor :type Actor%20Object%20Reference) (OtherComp :type Primitive%20Component%20Object%20Reference) (OtherBodyIndex :type Integer) (bFromSweep :type Boolean) (SweepResult :type Hit%20Result%20Structure%20%28by%20ref%29))
  (bind _asbp_player_ship_visuals (Utilities|Casting|CastToBP_PlayerShip_visuals OtherActor))
  (Variables|Default|SetBase%20Visuals%20Reference _asbp_player_ship_visuals)
  (Variables|Default|SetBase%20Logic%20Reference (Variables|/Game/Blueprints/Player/BP_PlayerShip_visuals.BP_PlayerShip_visuals_C|GetLogic%20Reference (Variables|Default|GetBase%20Visuals%20Reference)))
  (Utilities|FlowControl|Sequence
    (:then_0
      (CallFunction|CustomPowerUpLogic)
      (Game|SpawnActorfromClass (Variables|Default|GetParticle) (Transformation|GetWorldTransform (Variables|Default|GetDefaultSceneRoot)) "AlwaysSpawn" 0 0))
    (:then_1
      ;[1 0.4837 0.04957] Turn Off
      (if (Variables|Default|GetHave%20A%20Duration)
        (Rendering|SetVisibility (Variables|Default|GetMesh) false false)
        (Variables|/Script/Engine.PrimitiveComponent|SetbGenerateOverlapEvents (Variables|Default|GetCollider) false)
        (Utilities|FlowControl|Delay (Variables|Default|GetDuration))
        (CallFunction|PowerUpEndLogic))
      (Actor|DestroyActor))))

(event EventBeginPlay
  (Class|ActorSequenceComponent|PlaySequence (Variables|Default|GetFloat%20Animation)))

(fn ConstructionScript)

(fn CustomPowerUpLogic
  (return))

(fn PowerUpEndLogic)